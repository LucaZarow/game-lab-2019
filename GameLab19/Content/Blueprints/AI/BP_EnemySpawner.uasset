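; Enemy spawner Blueprint that creates one AI enemy of a selected type each time its SpawnEnemy event runs.
; A switch on AICharacter picks the pawn class: dummy, creep, archer, toxic or whirlwind.
; All branches share one SpawnAIFromClass call at the SpawnVolume's location and rotation, then copy the spawner's Tags onto the new pawn.
; A random-point-in-volume node is present but unused, so spawns do not scatter.
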(event `SpawnEnemy`
  (switch `/Game/Blueprints/AI/AI_Character` (`self.AI_Character`)
    (:`NewEnumerator0`
      (set `self.AI_Class` "/Game/Blueprints/AI/AI_Characters/AI_Character_0.AI_Character_0_C"))
    (:`NewEnumerator4`
      (set `self.AI_Class` "/Game/Blueprints/AI/AI_Characters/BP_AI_BasicCreep.BP_AI_BasicCreep_C"))
    (:`NewEnumerator1`
      (set `self.AI_Class` "/Game/Blueprints/AI/AI_Characters/BP_AI_BetaArcher.BP_AI_BetaArcher_C"))
    (:`NewEnumerator2`
      (set `self.AI_Class` "/Game/Blueprints/AI/AI_Characters/BP_AI_Character_Toxic.BP_AI_Character_Toxic_C"))
    (:`NewEnumerator3`
      (set `self.AI_Class` "/Game/Blueprints/AI/AI_Characters/BP_AI_WhirlWind.BP_AI_WhirlWind_C")))
  (bind _returnvalue (`AIBlueprintHelperLibrary.SpawnAIFromClass` (`self.AI_Class`) null (`SceneComponent.K2_GetComponentLocation` (`self.SpawnVolume`)) (`SceneComponent.K2_GetComponentRotation` (`self.SpawnVolume`))))
  (set `Actor.Tags` (`self.Tags`) _returnvalue))

(fn `UserConstructionScript`)