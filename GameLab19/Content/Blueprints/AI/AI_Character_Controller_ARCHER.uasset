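; AI controller for the Chad and Beta archer enemies, running the archer behavior tree when it possesses either pawn type.
; AI perception updates for the Pierre player character set the CanSeePlayer blackboard key from whether the stimulus was sensed.
; The same update calls StartFiring or StopFiring directly on the possessed archer, casting to each archer class in turn.
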(event `self.OnPossess`
  (params (PossessedPawn :type "Pawn Object Reference"))
  (cast `/Game/Blueprints/AI/BP_AI_ChadArcher` PossessedPawn
    (:`then`
      _)
    (:`CastFailed`
      (cast `/Game/Blueprints/AI/BP_AI_BetaArcher` PossessedPawn)))
  (`self.RunBehaviorTree` "/Game/AI/AI_BT_Archer.AI_BT_Archer"))

(event `self.AIPerception.OnTargetPerceptionUpdated`
  (params (Actor :type "Actor Object Reference") (Stimulus :type "AIStimulus Structure"))
  (bind (_age _expirationage _strength _stimuluslocation _receiverlocation _tag _bsuccessfullysensed) (break `AIStimulus` Stimulus))
  (bind _returnvalue (`self.K2_GetPawn`))
  (`KismetSystemLibrary.PrintString` "Perceving Target")
  (cast `/Game/Blueprints/Attacking_Testing/BP_Player_Pierre` Actor
    (:`then`
      (`BlackboardComponent.SetValueAsBool` (`AIBlueprintHelperLibrary.GetBlackboard` null) "CanSeePlayer" _bsuccessfullysensed)
      (if _bsuccessfullysensed
        (bind _asbp_ai_chad_archer (cast `/Game/Blueprints/AI/BP_AI_ChadArcher` _returnvalue)
          (:`then`
            (`/Game/Blueprints/AI/BP_AI_ChadArcher.StartFiring` _asbp_ai_chad_archer))
          (:`CastFailed`
            (bind _asbp_ai_beta_archer (cast `/Game/Blueprints/AI/BP_AI_BetaArcher` _returnvalue))
            (`/Game/Blueprints/AI/BP_AI_BetaArcher.StartFiring` _asbp_ai_beta_archer)))
        (else
          (bind _asbp_ai_chad_archer_2 (cast `/Game/Blueprints/AI/BP_AI_ChadArcher` _returnvalue)
            (:`then`
              (`/Game/Blueprints/AI/BP_AI_ChadArcher.StopFiring` _asbp_ai_chad_archer_2))
            (:`CastFailed`
              (bind _asbp_ai_beta_archer_2 (cast `/Game/Blueprints/AI/BP_AI_BetaArcher` _returnvalue))
              (`/Game/Blueprints/AI/BP_AI_BetaArcher.StopFiring` _asbp_ai_beta_archer_2))))))
    (:`CastFailed`
      (`KismetSystemLibrary.PrintString` "Casting failed"))))

(fn `UserConstructionScript`
  (`parent.UserConstructionScript`))