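; AI archer Blueprint that repeatedly fires a three-projectile spread.
; StartFiring runs FireWeapon on a looping timer paced by RangeAttackSpeed, and StopFiring clears it.
; Each volley spawns Test_Projectile at the actor's transform and at ten degrees of yaw to either side, passing CharcterType as AttackerType.
; The negative-yaw shot zeroes pitch, while the other two keep the actor's pitch.
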(event `StartFiring`
  (`KismetSystemLibrary.K2_SetTimer` null "FireWeapon" (`self.Range_AttackSpeed`) true))

(event `self.ReceiveBeginPlay`)

(event `StopFiring`
  (`KismetSystemLibrary.K2_ClearTimer` null "FireWeapon"))

(event `FireWeapon`
  (bind _returnvalue (`self.GetTransform`))
  (bind _charctertype (`self.CharcterType`))
  (bind _location (.location _returnvalue))
  (bind _rotation (.rotation _returnvalue))
  (bind _scale (.scale _returnvalue))
  (`|SpawnActorFromClass` "/Game/Blueprints/Attacking_Testing/Test_Projectile.Test_Projectile_C" _returnvalue "AlwaysSpawn" "OverrideRootScale" null 6 _charctertype false null)
  (`|SpawnActorFromClass` "/Game/Blueprints/Attacking_Testing/Test_Projectile.Test_Projectile_C" (`KismetMathLibrary.MakeTransform` _location (`KismetMathLibrary.MakeRotator` (.roll _rotation) 0.0 (- (.yaw _rotation) 10.0)) _scale) "AlwaysSpawn" "OverrideRootScale" null 6 _charctertype false null)
  (`|SpawnActorFromClass` "/Game/Blueprints/Attacking_Testing/Test_Projectile.Test_Projectile_C" (`KismetMathLibrary.MakeTransform` _location (`KismetMathLibrary.MakeRotator` (.roll _rotation) (.pitch _rotation) (+ (.yaw _rotation) 10.0)) _scale) "AlwaysSpawn" "OverrideRootScale" null 6 _charctertype false null))

(fn `UserConstructionScript`)