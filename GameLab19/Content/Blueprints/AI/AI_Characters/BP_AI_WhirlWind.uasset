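; Whirlwind AI enemy, a child character that sets its AI type and attacks with a spinning melee move.
; TurnonMelee and TurnOffMelee start and clear a looping AttackAction timer paced by MeleeAttackSpeed.
; Each attack halts movement, spawns a large launching, staggering sphere hitbox, and spins the mesh on Tick for SpinDuration before restoring animation and movement.
; Damage and death extend parent logic with random beast sounds, plus a particle effect on death.
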(event `self.TurnOnMelee`
  (if (not (`KismetSystemLibrary.K2_IsTimerActive` null "AttackAction"))
    (`KismetSystemLibrary.K2_SetTimer` null "AttackAction" (`self.Melee_AttackSpeed`) true)))

(event `self.TurnOffMelee`
  (`KismetSystemLibrary.K2_ClearTimer` null "AttackAction"))

(event `AttackAction`
  ;[1 1 1] AttackAction
  (set `self.canMove` false)
  (`|ExecutionSequence`
    (:`then_0`
      (`|SpawnActorFromClass` "/Game/Blueprints/Combat_System/BP_Hitbox_Sphere.BP_Hitbox_Sphere_C" (`KismetMathLibrary.MakeTransform` (`KismetMathLibrary.MakeVector` 0.0 0.0 15.0) (struct) (6.0 6.0 6.0)) "Undefined" "OverrideRootScale" self self 1.0 (`self.Melee_Damage`) (`self.CharcterType`) true 5000 true "NewEnumerator0" null))
    (:`then_1`
      (`SkeletalMeshComponent.PlayAnimation` (`self.Mesh`) "/Game/Assets/Characters/WhirlWindDemon/Whirlwind_ArmsLift_Anim.Whirlwind_ArmsLift_Anim" false)
      (`GameplayStatics.PlaySoundAtLocation` null (`self.K2_GetActorLocation`) (struct) 1.0 1.0 0.0 null null self)
      (set `self.spin` true)
      (`KismetSystemLibrary.Delay` (`self.SpinDuration`))
      (set `self.spin` false)
      (`SceneComponent.K2_SetRelativeRotation` (`self.Mesh`) (struct :`Yaw` -90.0) false false)
      (set `self.canMove` true)
      (`SkeletalMeshComponent.SetAnimationMode` (`self.Mesh`) "AnimationBlueprint"))))

(event `self.ReceiveTick`
  (params (DeltaSeconds :type "Float (single-precision)"))
  (if (`self.spin`)
    (`SceneComponent.K2_AddLocalRotation` (`self.Mesh`) (`KismetMathLibrary.MakeRotator` 0.0 0.0 (* DeltaSeconds 1000.0)) false false)))

(event `self.Death`
  (bind _returnvalue (`self.K2_GetActorLocation`))
  (if (<= (`KismetMathLibrary.RandomFloat`) 0.5)
    (`GameplayStatics.PlaySoundAtLocation` "/Game/Assets/Audio/SoundEffects/Monster/Beast_Death_2.Beast_Death_2" _returnvalue (struct) 0.7 1.0 0.0 null null self)
    (else
      (`GameplayStatics.PlaySoundAtLocation` "/Game/Assets/Audio/SoundEffects/Monster/Beast_Death_3.Beast_Death_3" _returnvalue (struct) 0.7 1.0 0.0 null null self)))
  (`GameplayStatics.SpawnEmitterAtLocation` "/Game/ParticleEffects/Death_Creep.Death_Creep" _returnvalue)
  (`parent.Death`))

(fn `Damaged`
  (params (Damage :type Integer) (DamageType :type "/Game/Blueprints/Combat_System/CharacterType Enum" :default "NewEnumerator0") (attackorigine :type "/Game/Blueprints/Combat_System/AttackOrigine Enum" :default "NewEnumerator0"))
  (returns (HasDamaged :type Boolean))
  (bind _returnvalue (`self.K2_GetActorLocation`))
  (bind _hasdamaged (`parent.Damaged` Damage DamageType attackorigine))
  (if _hasdamaged
    (if (<= (`KismetMathLibrary.RandomFloat`) 0.5)
      (`GameplayStatics.PlaySoundAtLocation` "/Game/Assets/Audio/SoundEffects/Monster/Beast_2.Beast_2" _returnvalue (struct) 0.7 1.0 0.0 null null self)
      (else
        (`GameplayStatics.PlaySoundAtLocation` "/Game/Assets/Audio/SoundEffects/Monster/Beast_3.Beast_3" _returnvalue (struct) 0.7 1.0 0.0 null null self)))
    (return _hasdamaged)))

(fn `UserConstructionScript`
  (set `self.AiCharacter` "NewEnumerator3")
  (`parent.UserConstructionScript`))