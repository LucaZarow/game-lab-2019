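; BP_AI_BetaArcher is an AI archer character that fires projectiles on a looping timer while its ranged attack is on.
; TurnonRange starts the timer; TurnOffMelee, despite its name, clears it.
; Each shot plays the bow animation, waits to spawn a Test_Projectile tagged with the character's type, then restores the Animation Blueprint.
; CalcArrowPosition offsets the actor's location by RelativeArrowPos in world space, ignoring facing.
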(event `self.TurnOnRange`
  (set `self.IsShooting` true)
  (`KismetSystemLibrary.K2_SetTimer` null "FireWeapon" (`self.Range_AttackSpeed`) true))

(event `FireWeapon`
  (`SkeletalMeshComponent.PlayAnimation` (`self.Mesh`) "/Game/Assets/Characters/ArcherDemon/Archer_And_Bow_Shoot.Archer_And_Bow_Shoot" false)
  (`KismetSystemLibrary.Delay` 1.33)
  (bind _output_get (`self.CalcArrowPosition`))
  (`|SpawnActorFromClass` "/Game/Blueprints/Combat_System/Projectiles/Test_Projectile.Test_Projectile_C" _output_get "AlwaysSpawn" "OverrideRootScale" null 6 (`self.CharcterType`) false 0 null)
  (`SkeletalMeshComponent.SetAnimationMode` (`self.Mesh`) "AnimationBlueprint"))

(event `self.TurnOffMelee`
  (set `self.IsShooting` false)
  (`KismetSystemLibrary.K2_ClearTimer` null "FireWeapon"))

(fn `CalcArrowPosition`
  (returns (Output_Get :type "Transform Structure"))
  (bind _output_get (set `self.Transform` (`self.GetTransform`)))
  (bind _output_get_2 (set `self.Transform` (`KismetMathLibrary.MakeTransform` (+ (.location _output_get) (`self.RelativeArrowPos`)) (.rotation _output_get) (.scale _output_get))))
  (return _output_get_2))

(fn `UserConstructionScript`)