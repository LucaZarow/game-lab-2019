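; BP_AI_Tutorial is an AI character, named for the tutorial, that sets its character type and builds on a parent AI class.
; Turning melee on starts a looping timer that spawns BP_Hitbox_Cube with damage, launch and stagger; turning it off clears the timer.
; Its Damaged override prints the attack origin and passes zero damage to the parent for one origin type, forwarding others unchanged.
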(event `self.ReceiveTick`
  (params (DeltaSeconds :type "Float (single-precision)")))

(event `self.TurnOnMelee`
  (if (not (`KismetSystemLibrary.K2_IsTimerActive` null "AttackAction"))
    (`KismetSystemLibrary.K2_SetTimer` null "AttackAction" (`self.Melee_AttackSpeed`) true)))

(event `self.TurnOffMelee`
  (`KismetSystemLibrary.K2_ClearTimer` null "AttackAction"))

(event `AttackAction`
  ;[1 1 1] AttackAction
  (`|SpawnActorFromClass` "/Game/Blueprints/Combat_System/BP_Hitbox_cUBE.BP_Hitbox_Cube_C" (`KismetMathLibrary.MakeTransform` (`KismetMathLibrary.MakeVector` 100.0 0.0 (`CapsuleComponent.CapsuleHalfHeight` (`self.CapsuleComponent`)))) "AlwaysSpawn" "OverrideRootScale" self self 0.2 false (`self.Melee_Damage`) (`self.CharcterType`) true 5000 true null))

(fn `Damaged`
  (params (Damage :type Integer) (DamageType :type "/Game/Blueprints/Combat_System/CharacterType Enum" :default "NewEnumerator0") (attackorigine :type "/Game/Blueprints/Combat_System/AttackOrigine Enum" :default "NewEnumerator0"))
  (returns (HasDamaged :type Boolean))
  (`KismetSystemLibrary.PrintString` (`|GetEnumeratorNameAsString` attackorigine))
  (if (`|EnumEquality` attackorigine "NewEnumerator0")
    (bind _hasdamaged (`parent.Damaged` 0 "NewEnumerator1" attackorigine))
    (return _hasdamaged)
    (else
      (bind _hasdamaged_2 (`parent.Damaged` Damage DamageType attackorigine))
      (return _hasdamaged_2))))

(fn `UserConstructionScript`
  (set `self.AiCharacter` "NewEnumerator4")
  (`parent.UserConstructionScript`))