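; Basic creep AI character that performs a repeating melee attack while melee is switched on.
; TurnOnMelee_1 starts a looping AttackAction timer at MeleeAttackSpeed unless already running, printing the timer state for debugging, and TurnOffMelee_1 clears it.
; Each AttackAction spawns a BP_Hitbox_Real owned by the creep, passing a fixed forward/capsule-height offset transform, melee damage, attacker type and launch power.
; Unconnected IsShooting toggles remain in the graph.
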(event `TurnOnMelee_1`
  (bind _returnvalue (`KismetSystemLibrary.K2_IsTimerActive` null "AttackAction"))
  (`KismetSystemLibrary.PrintString` (`KismetStringLibrary.Conv_BoolToString` _returnvalue))
  (if (not _returnvalue)
    (`KismetSystemLibrary.K2_SetTimer` null "AttackAction" (`self.Melee_AttackSpeed`) true)))

(event `TurnOffMelee_1`
  (`KismetSystemLibrary.K2_ClearTimer` null "AttackAction"))

(event `AttackAction`
  ;[1 1 1] AttackAction
  (`|SpawnActorFromClass` "/Game/Blueprints/Combat_System/BP_Hitbox_Real.BP_Hitbox_Real_C" (`KismetMathLibrary.MakeTransform` (`KismetMathLibrary.MakeVector` 100.0 0.0 (`CapsuleComponent.CapsuleHalfHeight` (`self.CapsuleComponent`)))) "AlwaysSpawn" "OverrideRootScale" self self 0.2 (`self.Melee_Damage`) (`self.CharcterType`) true 5000 null))

(fn `UserConstructionScript`)