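; BP_AI_Character_Toxic is an AI character variant that emits a repeating area-damage hitbox.
; On BeginPlay it starts a looping timer at MeleeAttackSpeed that spawns an enlarged BP_Hitbox_Sphere carrying melee damage and lasting one interval.
; The spawn transform is a fixed near-origin location, with the character passed as owner and spawner.
; Launch and stagger events are empty, and the construction script sets the character type enum.
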(event `self.GetLaunched`
  (params (Launcher :type "Actor Object Reference") (Launch_Force :type Integer)))

(event `self.ReceiveBeginPlay`
  (`parent.ReceiveBeginPlay`)
  (`KismetSystemLibrary.K2_SetTimerDelegate` (delegate `Attack`) (`self.Melee_AttackSpeed`) true))

(event `self.Stagger`)

(event `self.StaggeringProjectile`)

(event `Attack`
  (`KismetSystemLibrary.PrintString` "Hitbox spawn")
  (`|SpawnActorFromClass` "/Game/Blueprints/Combat_System/BP_Hitbox_Sphere.BP_Hitbox_Sphere_C" (`KismetMathLibrary.MakeTransform` (0.0 0.0 1.0) (struct) (4.0 4.0 4.0)) "AlwaysSpawn" "OverrideRootScale" self self (`self.Melee_AttackSpeed`) (`self.Melee_Damage`) (`self.CharcterType`) false 0 false null))

(fn `UserConstructionScript`
  (set `self.AiCharacter` "NewEnumerator2")
  (`parent.UserConstructionScript`))