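; BP_AI_ChadArcher is an AI archer character that attacks with a three-projectile spread.
; FireWeapon spawns three Test_Projectile actors at the actor's location: one along its facing and two yawed ten degrees to either side, each tagged with the character's type as attacker.
; The construction script attaches the Bow0 component to a left middle-finger socket on the mesh.
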(event `FireWeapon`
  (bind _returnvalue (`self.GetTransform`))
  (bind _charctertype (`self.CharcterType`))
  (bind _location (.location _returnvalue))
  (bind _rotation (.rotation _returnvalue))
  (bind _scale (.scale _returnvalue))
  (`|SpawnActorFromClass` "/Game/Blueprints/Combat_System/Projectiles/Test_Projectile.Test_Projectile_C" _returnvalue "AlwaysSpawn" "OverrideRootScale" null 6 _charctertype false 0 null)
  (`|SpawnActorFromClass` "/Game/Blueprints/Combat_System/Projectiles/Test_Projectile.Test_Projectile_C" (`KismetMathLibrary.MakeTransform` _location (`KismetMathLibrary.MakeRotator` (.roll _rotation) 0.0 (- (.yaw _rotation) 10.0)) _scale) "AlwaysSpawn" "OverrideRootScale" null 6 _charctertype false 0 null)
  (`|SpawnActorFromClass` "/Game/Blueprints/Combat_System/Projectiles/Test_Projectile.Test_Projectile_C" (`KismetMathLibrary.MakeTransform` _location (`KismetMathLibrary.MakeRotator` (.roll _rotation) (.pitch _rotation) (+ (.yaw _rotation) 10.0)) _scale) "AlwaysSpawn" "OverrideRootScale" null 6 _charctertype false 0 null))

(fn `UserConstructionScript`
  (`SceneComponent.K2_AttachToComponent` (`self.Bow_0`) (`self.Mesh`) "MiddleFinger1_L" "KeepRelative" "KeepRelative" "KeepRelative" true))