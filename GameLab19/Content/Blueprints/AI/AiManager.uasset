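; AI manager that tracks enemies in per-type lists (Creep, Archer, Toxic, Whirlwind) and caps how many of each share the active combat status.
; AddAiCharacter files an enemy by type and re-runs ActivateCharacter for that type, while RemoveAiCharacter only removes it from its list.
; ActivateCharacter sets BaseEnemy CombatStatus by list index, giving those under the type's max one status and the rest another.
; ActivateAIs refreshes all four types; Notify prints list counts.
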(event `ActivateAIs`
  (`|ExecutionSequence`
    (:`then_0`
      (`self.ActivateCharacter` "NewEnumerator4"))
    (:`then_1`
      (`self.ActivateCharacter` "NewEnumerator1"))
    (:`then_2`
      (`self.ActivateCharacter` "NewEnumerator2"))
    (:`then_3`
      (`self.ActivateCharacter` "NewEnumerator3"))))

(event `Notify`
  ;[1 1 1] prints number of AI for each
  (`KismetSystemLibrary.PrintString` (`KismetStringLibrary.Concat_StrStr` "Number of Basic is " (`KismetStringLibrary.Conv_IntToString` (`KismetArrayLibrary.Array_Length` (`.List_3_AF8C3D384AAA7BF7E4153B93A13BFF35` (break `/DatasmithContent/Blueprints/FBXImporter/ArrayOfActor` (`self.Basics`)))))))
  (`KismetSystemLibrary.PrintString` (`KismetStringLibrary.Concat_StrStr` "Number of Archers is " (`KismetStringLibrary.Conv_IntToString` (`KismetArrayLibrary.Array_Length` (`.List_3_AF8C3D384AAA7BF7E4153B93A13BFF35` (break `/DatasmithContent/Blueprints/FBXImporter/ArrayOfActor` (`self.Archers`)))))))
  (`KismetSystemLibrary.PrintString` (`KismetStringLibrary.Concat_StrStr` "Number of Toxics is " (`KismetStringLibrary.Conv_IntToString` (`KismetArrayLibrary.Array_Length` (`.List_3_AF8C3D384AAA7BF7E4153B93A13BFF35` (break `/DatasmithContent/Blueprints/FBXImporter/ArrayOfActor` (`self.Toxics`)))))))
  (`KismetSystemLibrary.PrintString` (`KismetStringLibrary.Concat_StrStr` "Number of Whirlwinds is " (`KismetStringLibrary.Conv_IntToString` (`KismetArrayLibrary.Array_Length` (`.List_3_AF8C3D384AAA7BF7E4153B93A13BFF35` (break `/DatasmithContent/Blueprints/FBXImporter/ArrayOfActor` (`self.Whirlwids`))))))))

(fn `ActivateArchers`
  (for (_array_element _array_index) (`.List_3_AF8C3D384AAA7BF7E4153B93A13BFF35` (break `/DatasmithContent/Blueprints/FBXImporter/ArrayOfActor` (`self.Archers`)))
    (if (< _array_index (`self.MaxArchers`))
      (bind _asbase_enemy (cast `/Game/Blueprints/Combat_System/BaseEnemy` _array_element)
        (:`then`
          (set `/Game/Blueprints/Combat_System/BaseEnemy.CombatStatus` "NewEnumerator0" _asbase_enemy))
        (:`CastFailed`
          (`KismetSystemLibrary.PrintString` "Archer Status change failed" :!label _label)))
      (else
        (bind _asbase_enemy_2 (cast `/Game/Blueprints/Combat_System/BaseEnemy` _array_element)
          (:`then`
            (set `/Game/Blueprints/Combat_System/BaseEnemy.CombatStatus` "NewEnumerator2" _asbase_enemy_2))
          (:`CastFailed`
            (goto _label)))))))

(fn `ActivateCharacter`
  (params (AiChara :type "/Game/Blueprints/AI/AI_Character Enum" :default "NewEnumerator0"))
  (switch `/Game/Blueprints/AI/AI_Character` AiChara
    (:`NewEnumerator4`
      (for (_array_element _array_index) (`.List_3_AF8C3D384AAA7BF7E4153B93A13BFF35` (break `/DatasmithContent/Blueprints/FBXImporter/ArrayOfActor` (`self.Basics`)))
        (if (< _array_index (`self.MaxBasics`))
          (bind _asbase_enemy (cast `/Game/Blueprints/Combat_System/BaseEnemy` _array_element)
            (:`then`
              (set `/Game/Blueprints/Combat_System/BaseEnemy.CombatStatus` "NewEnumerator0" _asbase_enemy))
            (:`CastFailed`
              (`KismetSystemLibrary.PrintString` "Basic Status change failed" :!label _label)))
          (else
            (bind _asbase_enemy_2 (cast `/Game/Blueprints/Combat_System/BaseEnemy` _array_element)
              (:`then`
                (set `/Game/Blueprints/Combat_System/BaseEnemy.CombatStatus` "NewEnumerator1" _asbase_enemy_2))
              (:`CastFailed`
                (goto _label)))))))
    (:`NewEnumerator1`
      (for (_array_element_2 _array_index_2) (`.List_3_AF8C3D384AAA7BF7E4153B93A13BFF35` (break `/DatasmithContent/Blueprints/FBXImporter/ArrayOfActor` (`self.Archers`)))
        (if (< _array_index_2 (`self.MaxArchers`))
          (bind _asbase_enemy_3 (cast `/Game/Blueprints/Combat_System/BaseEnemy` _array_element_2)
            (:`then`
              (set `/Game/Blueprints/Combat_System/BaseEnemy.CombatStatus` "NewEnumerator0" _asbase_enemy_3))
            (:`CastFailed`
              (`KismetSystemLibrary.PrintString` "Archer Status change failed" :!label _label_2)))
          (else
            (bind _asbase_enemy_4 (cast `/Game/Blueprints/Combat_System/BaseEnemy` _array_element_2)
              (:`then`
                (set `/Game/Blueprints/Combat_System/BaseEnemy.CombatStatus` "NewEnumerator1" _asbase_enemy_4))
              (:`CastFailed`
                (goto _label_2)))))))
    (:`NewEnumerator2`
      (for (_array_element_3 _array_index_3) (`.List_3_AF8C3D384AAA7BF7E4153B93A13BFF35` (break `/DatasmithContent/Blueprints/FBXImporter/ArrayOfActor` (`self.Toxics`)))
        (if (< _array_index_3 (`self.MaxToxics`))
          (bind _asbase_enemy_5 (cast `/Game/Blueprints/Combat_System/BaseEnemy` _array_element_3)
            (:`then`
              (set `/Game/Blueprints/Combat_System/BaseEnemy.CombatStatus` "NewEnumerator0" _asbase_enemy_5))
            (:`CastFailed`
              (`KismetSystemLibrary.PrintString` "Archer Status change failed" :!label _label_3)))
          (else
            (bind _asbase_enemy_6 (cast `/Game/Blueprints/Combat_System/BaseEnemy` _array_element_3)
              (:`then`
                (set `/Game/Blueprints/Combat_System/BaseEnemy.CombatStatus` "NewEnumerator1" _asbase_enemy_6))
              (:`CastFailed`
                (goto _label_3)))))))
    (:`NewEnumerator3`
      (for (_array_element_4 _array_index_4) (`.List_3_AF8C3D384AAA7BF7E4153B93A13BFF35` (break `/DatasmithContent/Blueprints/FBXImporter/ArrayOfActor` (`self.Whirlwids`)))
        (if (< _array_index_4 (`self.MaxWhirlwinds`))
          (bind _asbase_enemy_7 (cast `/Game/Blueprints/Combat_System/BaseEnemy` _array_element_4)
            (:`then`
              (set `/Game/Blueprints/Combat_System/BaseEnemy.CombatStatus` "NewEnumerator0" _asbase_enemy_7))
            (:`CastFailed`
              (`KismetSystemLibrary.PrintString` "Archer Status change failed" :!label _label_4)))
          (else
            (bind _asbase_enemy_8 (cast `/Game/Blueprints/Combat_System/BaseEnemy` _array_element_4)
              (:`then`
                (set `/Game/Blueprints/Combat_System/BaseEnemy.CombatStatus` "NewEnumerator1" _asbase_enemy_8))
              (:`CastFailed`
                (goto _label_4)))))))))

(fn `AddAiCharacter`
  (params (AI :type "/Game/Blueprints/Combat_System/BaseEnemy Object Reference"))
  (bind _aicharacter (`/Game/Blueprints/Combat_System/BaseEnemy.AiCharacter` AI))
  (switch `/Game/Blueprints/AI/AI_Character` _aicharacter
    (:`NewEnumerator0`
      (`KismetSystemLibrary.PrintString` "Unrecinized AI do nothing"))
    (:`NewEnumerator4`
      (`KismetArrayLibrary.Array_Add` (`.List_3_AF8C3D384AAA7BF7E4153B93A13BFF35` (break `/DatasmithContent/Blueprints/FBXImporter/ArrayOfActor` (`self.Basics`))) AI)
      (`self.ActivateCharacter` _aicharacter :!label _label))
    (:`NewEnumerator1`
      (`KismetArrayLibrary.Array_Add` (`.List_3_AF8C3D384AAA7BF7E4153B93A13BFF35` (break `/DatasmithContent/Blueprints/FBXImporter/ArrayOfActor` (`self.Archers`))) AI)
      (goto _label))
    (:`NewEnumerator2`
      (`KismetArrayLibrary.Array_Add` (`.List_3_AF8C3D384AAA7BF7E4153B93A13BFF35` (break `/DatasmithContent/Blueprints/FBXImporter/ArrayOfActor` (`self.Toxics`))) AI)
      (goto _label))
    (:`NewEnumerator3`
      (`KismetArrayLibrary.Array_Add` (`.List_3_AF8C3D384AAA7BF7E4153B93A13BFF35` (break `/DatasmithContent/Blueprints/FBXImporter/ArrayOfActor` (`self.Whirlwids`))) AI)
      (goto _label))
    (:`NewEnumerator5`
      (`KismetSystemLibrary.PrintString` "No AI inputed"))))

(fn `RemoveAiCharacter`
  (params (CharacterType :type "/Game/Blueprints/AI/AI_Character Enum" :default "NewEnumerator0") (Enemy :type "/Game/Blueprints/Combat_System/BaseCharacter Object Reference"))
  (switch `/Game/Blueprints/AI/AI_Character` CharacterType
    (:`NewEnumerator0`
      (`KismetSystemLibrary.PrintString` "Unrecinized AI do nothing"))
    (:`NewEnumerator4`
      (`KismetArrayLibrary.Array_RemoveItem` (`.List_3_AF8C3D384AAA7BF7E4153B93A13BFF35` (break `/DatasmithContent/Blueprints/FBXImporter/ArrayOfActor` (`self.Basics`))) Enemy))
    (:`NewEnumerator1`
      (`KismetArrayLibrary.Array_RemoveItem` (`.List_3_AF8C3D384AAA7BF7E4153B93A13BFF35` (break `/DatasmithContent/Blueprints/FBXImporter/ArrayOfActor` (`self.Archers`))) Enemy))
    (:`NewEnumerator2`
      (`KismetArrayLibrary.Array_RemoveItem` (`.List_3_AF8C3D384AAA7BF7E4153B93A13BFF35` (break `/DatasmithContent/Blueprints/FBXImporter/ArrayOfActor` (`self.Toxics`))) Enemy))
    (:`NewEnumerator3`
      (`KismetArrayLibrary.Array_RemoveItem` (`.List_3_AF8C3D384AAA7BF7E4153B93A13BFF35` (break `/DatasmithContent/Blueprints/FBXImporter/ArrayOfActor` (`self.Whirlwids`))) Enemy))
    (:`NewEnumerator5`
      (`KismetSystemLibrary.PrintString` "No AI inputed"))))

(fn `UserConstructionScript`)