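; BP_Damaging is a hit box actor that damages characters overlapping it.
; On overlap it calls Damaged on a BaseCharacter with its stored damage and attacker type.
; If the hit lands, it launches the character away using LaunchPower and staggers it when it is a BaseEnemy.
; SetStats lets the spawner or owner configure damage and attacker type.
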(event `self.ReceiveActorBeginOverlap`
  (params (OtherActor :type "Actor Object Reference"))
  ;[1 1 1] Apply damage to object
  (bind _asbase_character (cast `/Game/Blueprints/Combat_System/BaseCharacter` OtherActor))
  (bind _hasdamaged (`/Game/Blueprints/Combat_System/BaseCharacter.Damaged` _asbase_character (`self.HitBoxDamage`) (`self.AttackerType`)))
  (if _hasdamaged
    (`/Game/Blueprints/Combat_System/BaseCharacter.GetLaunched` _asbase_character self (`self.LaunchPower`))
    (bind _asbase_enemy (cast `/Game/Blueprints/Combat_System/BaseEnemy` OtherActor))
    (`/Game/Blueprints/Combat_System/BaseEnemy.Stagger` _asbase_enemy)))

(event `self.ReceiveActorEndOverlap`
  (params (OtherActor :type "Actor Object Reference")))

(fn `SetStats`
  (params (Damage :type Integer) (AttackType :type "/Game/Blueprints/Combat_System/CharacterType Enum" :default "NewEnumerator0"))
  (set `self.HitBoxDamage` Damage)
  (set `self.AttackerType` AttackType))

(fn `UserConstructionScript`)