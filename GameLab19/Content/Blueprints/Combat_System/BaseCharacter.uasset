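; Base character class for combat, giving player and enemy pawns shared health, damage, death, knockback and walk speed logic.
; Characters default to Enemy, and damage applies only when its type differs from the character's, with damaged enemies registered as the GameMode's current enemy.
; Heal and Damaged feed CalculateHealth, which clamps health and can trigger CheckDeath, calling an empty Death function.
; GetLaunched pushes the character horizontally away from the launcher.
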(fn `Calculate Health`
  (params (addition :type Integer))
  (bind _maxhealth (`self.MaxHealth`))
  (bind _output_get (set `self.CurrentHealth` (+ (`self.CurrentHealth`) addition)))
  (if (< _output_get 0)
    (set `self.CurrentHealth` 0)
    (`self.Check Death` :!label _label)
    (elif (> _output_get _maxhealth)
      (set `self.CurrentHealth` _maxhealth)
      (else
        (goto _label)))))

(fn `ChangeSpeed`
  (params (MaxWalkSpeed :type "Float (double-precision)"))
  (set `CharacterMovementComponent.MaxWalkSpeed` MaxWalkSpeed (`self.CharacterMovement`)))

(fn `Check Death`
  (if (<= (`self.CurrentHealth`) 0)
    (set `self.isDead` true)
    (`self.Death`)))

(fn `Damaged`
  (params (Damage :type Integer) (DamageType :type "/Game/Blueprints/Combat_System/CharacterType Enum" :default "NewEnumerator0"))
  (returns (HasDamaged :type Boolean))
  (if (`|EnumInequality` DamageType (`self.CharcterType`))
    (`self.Calculate Health` (* Damage -1))
    (switch `/Game/Blueprints/Combat_System/CharacterType` (`self.CharcterType`)
      (:`NewEnumerator0`
        _)
      (:`NewEnumerator1`
        (bind _asbp_game_mode (cast `/Game/Blueprints/BP_GameMode` (`GameplayStatics.GetGameMode`)))
        (`/Game/Blueprints/BP_GameMode.SetCurrentEnemy` _asbp_game_mode self)))
    (return true)
    (else
      (return false))))

(fn `Death`)

(fn `GetLaunched`
  (params (Launcher :type "Actor Object Reference") (Launch_Force :type Integer :default 0))
  (`MovementComponent.StopMovementImmediately` (`self.CharacterMovement`))
  (`self.LaunchCharacter` (* (`KismetMathLibrary.Normal` (`KismetMathLibrary.MakeVector` (.x (- (`self.K2_GetActorLocation`) (`self.K2_GetActorLocation` Launcher))) (.y (- (`self.K2_GetActorLocation`) (`self.K2_GetActorLocation` Launcher))))) Launch_Force) true))

(fn `Heal`
  (params (Healing :type Integer))
  (`self.Calculate Health` Healing))

(fn `UserConstructionScript`
  ;[1 1 1] Since most are enemies, only override player
  (set `self.CharcterType` "NewEnumerator1"))