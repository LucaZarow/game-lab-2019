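; Player character Blueprint handling movement and combat: melee hitbox, sword slash, orbiting ranged orb and dash.
; Movement uses world or camera-relative axes via ControlSwitch, alongside duplicate control-rotation handlers.
; BeginPlay attaches the orb to a Tick-rotated spring arm, and shoot axes aim and trigger it twin-stick style.
; Dash lerps the capsule forward by timeline with sweep, trail and cooldown, while Start/Stop events gate attack, slash and dash.
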(event `InputAxis|MoveForward`
  (params (AxisValue :type "Float (single-precision)"))
  (bind _controlswitch (`self.ControlSwitch`))
  ;[1 1 1] Basic Player Movement
  (`|ExecutionSequence`
    (:`then_0`
      (if _controlswitch
        (`self.AddMovementInput` (1.0 0.0 0.0) AxisValue)
        (else
          (`self.AddMovementInput` (`KismetMathLibrary.Normal` (`KismetMathLibrary.MakeVector` (.x (`SceneComponent.GetForwardVector` (`PlayerCameraManager.TransformComponent` (`GameplayStatics.GetPlayerCameraManager` 0)))) (.y (`SceneComponent.GetForwardVector` (`PlayerCameraManager.TransformComponent` (`GameplayStatics.GetPlayerCameraManager` 0)))))) AxisValue))))
    (:`then_1`
      (bind _returnvalue (`KismetMathLibrary.MakeVector` AxisValue (stale `InputAxis|MoveRight` AxisValue)))
      (if (> (`KismetMathLibrary.VSize` _returnvalue) 0.0) :!label _label
        (if _controlswitch
          _
          (else
            _))
        (`self.K2_SetActorRotation` (`KismetMathLibrary.Conv_VectorToRotator` _returnvalue) true)
        (`self.K2_AddActorWorldRotation` (`KismetMathLibrary.MakeRotator` 0.0 0.0 (.yaw (`SceneComponent.K2_GetComponentRotation` (`PlayerCameraManager.TransformComponent` (`GameplayStatics.GetPlayerCameraManager` 0))))))))))

(event `self.ReceiveBeginPlay`
  (bind _orbtemp (`self.OrbTemp`))
  ;[1 1 1] Spawn Ranged Orb Object
  (set `self.CanAttack` true)
  (set `self.CanSlash` true)
  (set `self.CanDash2` true)
  (`|ExecutionSequence`
    (:`then_0`
      (bind _returnvalue (`|SpawnActorFromClass` "/Game/Blueprints/RangedWeapon_Orb.RangedWeapon_Orb_C" (`SceneComponent.K2_GetComponentToWorld` _orbtemp) "Undefined" "OverrideRootScale" null null))
      (bind _output_get (set `self.Weapon_Orb` _returnvalue))
      (`self.K2_AttachToComponent` _output_get _orbtemp "None" "SnapToTarget" "SnapToTarget" "SnapToTarget" true))))

(event `InputAxis|MoveForward` :!enabledstate Disabled
  (params (AxisValue :type "Float (single-precision)"))
  ;[1 1 1] Basic Player Movement
  (`self.AddMovementInput` (`KismetMathLibrary.GetForwardVector` (`KismetMathLibrary.MakeRotator` 0.0 0.0 (.yaw (`self.GetControlRotation`)))) AxisValue))

(event `InputAxis|MoveRight`
  (params (AxisValue :type "Float (single-precision)"))
  ;[1 1 1] Basic Player Movement
  (`|ExecutionSequence`
    (:`then_0`
      (if (`self.ControlSwitch`)
        (`self.AddMovementInput` (0.0 1.0 0.0) AxisValue)
        (else
          (`self.AddMovementInput` (`KismetMathLibrary.Normal` (`KismetMathLibrary.MakeVector` (.x (`SceneComponent.GetRightVector` (`PlayerCameraManager.TransformComponent` (`GameplayStatics.GetPlayerCameraManager` 0)))) (.y (`SceneComponent.GetRightVector` (`PlayerCameraManager.TransformComponent` (`GameplayStatics.GetPlayerCameraManager` 0)))))) AxisValue))))
    (:`then_1`
      (goto _label))))

(event `self.ReceiveTick`
  (params (DeltaSeconds :type "Float (single-precision)"))
  ;[1 1 1] Rotatates Orb
  (`SceneComponent.K2_AddLocalRotation` (`self.SpringArm_Orb`) (`KismetMathLibrary.MakeRotator` 0.0 0.0 (* DeltaSeconds (`self.OrbRotationSpeed`))) false false))

(event `InputAxis|MoveRight` :!enabledstate Disabled
  (params (AxisValue :type "Float (single-precision)"))
  ;[1 1 1] Basic Player Movement
  (`self.AddMovementInput` (`KismetMathLibrary.GetRightVector` (`KismetMathLibrary.MakeRotator` 0.0 0.0 (.yaw (`self.GetControlRotation`)))) AxisValue))

(event `InputAxis|ShootUp`
  (params (AxisValue :type "Float (single-precision)"))
  (bind _weapon_orb (`self.Weapon_Orb`))
  ;[1 1 1] Ranged Attack 360 no scope
  (bind _returnvalue (`KismetMathLibrary.MakeVector` AxisValue (stale `InputAxis|ShootRight` AxisValue)))
  (if (> (`KismetMathLibrary.VSize` _returnvalue) 0.25) :!label _label_2
    (`/Game/Blueprints/RangedWeapon_Orb.PullTrigger` _weapon_orb (`KismetMathLibrary.Conv_VectorToRotator` _returnvalue))
    (else
      (`/Game/Blueprints/RangedWeapon_Orb.ReleaseTrigger` _weapon_orb))))

(event `InputAction|Attack`
  (params (Key :type "Key Structure"))
  ;[1 1 1] Attack
  (:`Pressed`
    (if (`self.CanAttack`)
      (`|SpawnActorFromClass` "/Game/Blueprints/Combat_System/BP_Hitbox_Real.BP_Hitbox_Real_C" (`KismetMathLibrary.Conv_VectorToTransform` (`SceneComponent.K2_GetComponentLocation` (`self.Mesh`))) "Undefined" "OverrideRootScale" null self (`self.Melee_Damage`) (`self.CharcterType`) false null))))

(event `Start Attack`
  ;[1 1 1] Attack
  (set `self.CanAttack` true))

(event `InputAxis|ShootRight`
  (params (AxisValue :type "Float (single-precision)"))
  ;[1 1 1] Ranged Attack 360 no scope
  (goto _label_2))

(event `Stop Attack`
  ;[1 1 1] Attack
  (set `self.CanAttack` false))

(event `InputAction|Slash`
  (params (Key :type "Key Structure"))
  ;[1 1 1] Slash
  (:`Pressed`
    (if (`self.CanSlash`)
      (`|SpawnActorFromClass` "/Game/Blueprints/Combat_System/BP_SwordSlash.BP_SwordSlash_C" (`KismetMathLibrary.Conv_VectorToTransform` (`SceneComponent.K2_GetComponentLocation` (`self.Mesh`))) "Undefined" "OverrideRootScale" null 0 "NewEnumerator0" false null))))

(event `Start Slash`
  ;[1 1 1] Slash
  (set `self.CanSlash` true))

(event `StopSlash`
  ;[1 1 1] Slash
  (set `self.CanSlash` false))

(event `StartDash`
  ;[1 1 1] Dash, Q key
  (set `self.CanDash2` true))

(event `InputAction|Dash`
  (params (Key :type "Key Structure"))
  ;[1 1 1] Dash, Q key
  (:`Pressed`
    (if (and (`self.CanDash2`) (`self.CanDash`))
      (`self.DashTrail`)
      (bind (_returnvalue _dashstartpos) (`self.CalcDashEndPos`))
      (`TimelineComponent.SetPlayRate` (`self.TimelineLerp`) (`self.DashSpeed`))
      (bind (_direction _newtrack_0) (`Timeline|TimelineLerp` :!via `PlayFromStart`)
        (:`Update`
          (`SceneComponent.K2_SetWorldLocation` (`self.CapsuleComponent`) (`KismetMathLibrary.VLerp` _dashstartpos _returnvalue _newtrack_0) true false)
          (set `self.CanDash` false)
          (`KismetSystemLibrary.Delay` 2.55)
          (set `self.CanDash` true))))))

(event `StopDash`
  ;[1 1 1] Dash, Q key
  (set `self.CanDash2` false))

(fn `CalcDashEndPos`
  (returns (ReturnValue :type "Vector Structure") (DashStartPos :type "Vector Structure"))
  (locals (`Dash Start Pos` :type "Vector Structure" :default (0.0 0.0 0.0)))
  (bind _dash_start_pos (`local.Dash Start Pos`))
  ;[1 1 1] Dash, on release of Q key
  (set `local.Dash Start Pos` (`SceneComponent.K2_GetComponentLocation` (`self.CapsuleComponent`)))
  (return (+ _dash_start_pos (* (`SceneComponent.GetForwardVector` (`self.CapsuleComponent`)) (`self.DashDistance`))) _dash_start_pos))

(fn `DashTrail`
  (`GameplayStatics.SpawnEmitterAttached` null (`self.Cylinder`)))

(fn `UserConstructionScript`)