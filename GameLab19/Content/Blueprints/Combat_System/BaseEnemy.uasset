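; BaseEnemy is the base enemy for the combat system, handling shared setup, stagger, death and AI manager registration.
; On BeginPlay it registers with the AiManager found by a world actor search and fills health.
; Timed events toggle a Staggered flag, immediately for projectiles or after a short delay otherwise; melee and range toggle events are empty stubs.
; Death unregisters the enemy, reports its wave to any linked altar, then destroys it.
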(event `Stagger`
  (`KismetSystemLibrary.Delay` 0.15)
  (set `self.Staggered` true)
  (`KismetSystemLibrary.Delay` 0.5)
  (set `self.Staggered` false))

(event `StaggeringProjectile`
  (set `self.Staggered` true)
  (`KismetSystemLibrary.Delay` 0.5)
  (set `self.Staggered` false))

(event `self.ReceiveBeginPlay`
  (`self.AddToAiManager`)
  (set `self.CharcterType` "NewEnumerator1")
  (set `self.CombatStatus` "NewEnumerator0")
  (set `self.CurrentHealth` (`self.MaxHealth`)))

(event `TurnOnMelee`)

(event `TurnOffMelee`)

(event `TurnOnRange`)

(event `TurnOffRange`)

(event `self.Death`
  (bind _altar_ref (`self.Altar_Ref`))
  (`self.RemoveFromAiManager` (`self.AiCharacter`))
  (set `self.isDead` true)
  (`/Engine/EditorBlueprintResources/StandardMacros.IsValid` _altar_ref
    (:`Is Valid`
      (`/Game/Blueprints/Checkpoint_System/Altar.enemyDeath` _altar_ref (`self.waveNumber`) self)
      (`/Game/Blueprints/Checkpoint_System/Altar.AltarKnowEnemyDeath` _altar_ref))
    (:`Is Not Valid`
      _))
  (`self.K2_DestroyActor`))

(fn `AddToAiManager`
  (bind _ai_manager (`self.GetAiManager`))
  (`/Game/Blueprints/AI/AiManager.AddAiCharacter` _ai_manager self))

(fn `GetAiManager`
  (returns (AI_Manager :type "/Game/Blueprints/AI/AiManager Object Reference"))
  (bind _outactors (`GameplayStatics.GetAllActorsOfClass` "/Game/Blueprints/AI/AiManager.AiManager_C"))
  (for _array_element _outactors
    (return _array_element))
  (return _array_element))

(fn `RemoveFromAiManager`
  (params (NewParam :type "/Game/Blueprints/AI/AI_Character Enum" :default "NewEnumerator0"))
  (bind _ai_manager (`self.GetAiManager`))
  (`/Game/Blueprints/AI/AiManager.RemoveAiCharacter` _ai_manager NewParam self))

(fn `UserConstructionScript`
  (set `self.CharcterType` "NewEnumerator1")
  (set `self.CombatStatus` "NewEnumerator0"))