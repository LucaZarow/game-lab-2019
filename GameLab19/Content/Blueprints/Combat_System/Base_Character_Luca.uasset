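; Base combat character that handles health, team-filtered damage and knockback, judging by its Player/Enemy character type.
; Heal and Damaged feed Calculate Health, which clamps the value and calls a death check that is currently a stub.
; Damaged ignores hits whose type matches the character's own, and damaged enemies register as the current enemy on UI_Test_GameMode.
; GetLaunched pushes the character away from the launcher; health bar creation is disconnected and disabled.
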(fn `Calculate Health`
  (params (addition :type Integer))
  (bind _maxhealth (`self.MaxHealth`))
  (bind _output_get (set `self.CurrentHealth` (+ (`self.CurrentHealth`) addition)))
  (if (< _output_get 0)
    (set `self.CurrentHealth` 0)
    (`self.Check Death` :!label _label)
    (elif (> _output_get _maxhealth)
      (set `self.CurrentHealth` _maxhealth)
      (else
        (goto _label)))))

(fn `Check Death`
  (if (<= (`self.CurrentHealth`) 0)
    _))

(fn `Damaged`
  (params (Damage :type Integer) (DamageType :type "/Game/Blueprints/Combat_System/CharacterType Enum" :default "NewEnumerator0"))
  (returns (HasDamaged :type Boolean))
  (if (`|EnumInequality` DamageType (`self.CharcterType`))
    (`self.Calculate Health` (* Damage -1))
    (switch `/Game/Blueprints/Combat_System/CharacterType` (`self.CharcterType`)
      (:`NewEnumerator0`
        _)
      (:`NewEnumerator1`
        (bind _asui_test_game_mode (cast `/Game/Blueprints/UI/UI_Test_GameMode` (`GameplayStatics.GetGameMode`)))
        (`/Game/Blueprints/UI/UI_Test_GameMode.SetCurrentEnemy` _asui_test_game_mode self)))
    (return true)
    (else
      (return false))))

(fn `GetLaunched`
  (params (Launcher :type "Actor Object Reference") (Launch_Force :type Integer :default 0))
  (`self.LaunchCharacter` (* (`KismetMathLibrary.Normal` (- (`self.K2_GetActorLocation`) (`self.K2_GetActorLocation` Launcher))) Launch_Force) true))

(fn `Heal`
  (params (Healing :type Integer))
  (`self.Calculate Health` Healing))

(fn `UserConstructionScript`)