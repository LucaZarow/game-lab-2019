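; AltarWaveCount is a checkpoint-system Blueprint that relates wave progress at an altar to a post-process scene colour tint.
; BeginPlay caches the settings and tint from a post-process volume.
; Waves builds new settings with a white tint whose alpha scales by the completed-wave fraction, but only stores them, never writing them back to the volume.
; The Enemies input is unused, and the event dispatcher binding never runs.
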(event `self.ReceiveBeginPlay`
  (bind _settings (`PostProcessVolume.Settings` (`self.PPVolume`)))
  (set `self.PPSettings` _settings)
  (set `self.colorTint` (`.SceneColorTint` (break `PostProcessSettings` _settings))))

(event `CustomEvent_0`)

(fn `waves`
  (params (waveNumber :type Integer) (totalNumOfWaves :type Integer) (enemies :type "Array of Pawn Object Reference"))
  (bind (_colortint_r _colortint_g _colortint_b _colortint_a) (break `LinearColor` (`self.colorTint`)))
  (set `self.fractionOfWaves` (/ (`KismetMathLibrary.Conv_IntToDouble` waveNumber) (`KismetMathLibrary.Conv_IntToDouble` totalNumOfWaves)))
  (set `self.PPSettings` (make `PostProcessSettings` :`SceneColorTint` (make `LinearColor` 1.0 1.0 1.0 (* _colortint_a (`self.fractionOfWaves`))))))