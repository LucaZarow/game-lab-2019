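; Checkpoint-system altar that drives enemy waves through a linked trigger spawner.
; NewWave records the wave number and enemies, setting a death threshold from group size.
; Tick polls the enemy count, requesting the next wave at that threshold or ending waves, without checking WavesInProgress.
; Post-process tint logic is unfinished, with a zero-by-zero wave fraction and several empty stub functions.
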(event `ColorEvent`
  (bind _settings (`PostProcessVolume.Settings` (`self.PPVolume`)))
  (set `self.PPSettings` _settings)
  (set `self.colorTint` (`.SceneColorTint` (break `PostProcessSettings` _settings))))

(event `WavesStart`
  (set `self.wavesInProgress` true))

(event `WavesEnd`
  (set `self.wavesInProgress` false))

(event `self.ReceiveTick`
  (params (DeltaSeconds :type "Float (single-precision)"))
  (if true
    (if (<= (`KismetArrayLibrary.Array_Length` (`self.curEnemies`)) (`self.deathThreshold`))
      (bind _result (`/Engine/EditorBlueprintResources/StandardMacros.IncrementInt` (`self.curWaveNumber`))
        (:`  `
          (if (< _result (`self.numWaves`))
            (`/Game/Blueprints/Checkpoint_System/EnemySpawnTrigger.NextWave` (`self.myTriggerSpawner`))
            (else
              (`self.WavesEnd`))))))))

(fn `enemyDeath`)

(fn `NewWave`
  (params (waveNum :type Integer) (enemies :type "Array of Pawn Object Reference"))
  (set `self.curWaveNumber` waveNum)
  (bind _output_get (set `self.curEnemies` enemies))
  (if (<= (`KismetArrayLibrary.Array_Length` _output_get) 3)
    (set `self.deathThreshold` 1)
    (else
      (set `self.deathThreshold` 2))))

(fn `ThresholdReached`)

(fn `UserConstructionScript`)

(fn `waves`
  (params (WaveNumber :type Integer) (TotalNumberOfWaves :type Integer) (Enemies :type "Array of Pawn Object Reference"))
  (bind (_colortint_r _colortint_g _colortint_b _colortint_a) (break `LinearColor` (`self.colorTint`)))
  (set `self.fractionOfWaves` (/ (`KismetMathLibrary.Conv_IntToDouble` 0) (`KismetMathLibrary.Conv_IntToDouble` 0)))
  (set `self.PPSettings` (make `PostProcessSettings` :`SceneColorTint` (make `LinearColor` 1.0 1.0 1.0 (* _colortint_a (`self.fractionOfWaves`))))))