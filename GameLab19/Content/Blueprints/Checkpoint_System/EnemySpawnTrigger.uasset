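; Checkpoint trigger that starts wave-based enemy spawning for its linked Altar the first time the player overlaps it.
; It registers itself and the wave count on the Altar, spawns the first wave, and exposes NextWave for later ones.
; Each Wave map entry lists enemy types, spawned with matching behavior trees at successive TargetPoints.
; Enemies receive Altar and wave references, and the accumulating list is passed to the Altar.
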(event `self.ReceiveActorBeginOverlap`
  (params (OtherActor :type "Actor Object Reference"))
  (cast `/Game/Blueprints/BP_Player` OtherActor)
  (`/Engine/EditorBlueprintResources/StandardMacros.DoOnce` false
    (:`Completed`
      (set `/Game/Blueprints/Checkpoint_System/Altar.myTriggerSpawner` self (`self.altar`))
      (`self.SetOnAltarNumberOfWaves`)
      ;[1 1 1] Spawn First Wave
      (bind _output_get (set `self.waveNumber` 0))
      (`self.SpawnWave` _output_get)
      (`/Game/Blueprints/Checkpoint_System/Altar.WavesStart` (`self.altar`)))))

(event `NextWave`
  (bind _result (`/Engine/EditorBlueprintResources/StandardMacros.IncrementInt` (`self.waveNumber`))
    (:`  `
      (`self.SpawnWave` _result))))

(fn `SetOnAltarNumberOfWaves`
  (bind _keys (`BlueprintMapLibrary.Map_Keys` (`self.wave`)))
  (set `/Game/Blueprints/Checkpoint_System/Altar.numWaves` (`KismetArrayLibrary.Array_Length` _keys) (`self.altar`)))

(fn `SpawnOneEnemy`
  (params (Location :type "Vector Structure") (AICharacter :type "/Game/Blueprints/AI/AI_Character Enum" :default "NewEnumerator0"))
  (returns (ReturnValue :type "Pawn Object Reference"))
  (switch `/Game/Blueprints/AI/AI_Character` AICharacter
    (:`NewEnumerator0`
      (set `self.AI_Class` "/Game/Blueprints/AI/AI_Characters/NotInUse/AI_Character_0.AI_Character_0_C")
      (set `self.BehaviorTree` "/Game/Blueprints/AI/Behavior_Trees/AI_BT.AI_BT"))
    (:`NewEnumerator4`
      (set `self.AI_Class` "/Game/Blueprints/AI/AI_Characters/BP_AI_BasicCreep.BP_AI_BasicCreep_C")
      (set `self.BehaviorTree` "/Game/Blueprints/AI/Behavior_Trees/AI_BT_BasicCreep.AI_BT_BasicCreep"))
    (:`NewEnumerator1`
      (set `self.AI_Class` "/Game/Blueprints/AI/AI_Characters/BP_AI_BetaArcher.BP_AI_BetaArcher_C")
      (set `self.BehaviorTree` "/Game/Blueprints/AI/Behavior_Trees/AI_BT_Archer.AI_BT_Archer"))
    (:`NewEnumerator2`
      (set `self.AI_Class` "/Game/Blueprints/AI/AI_Characters/BP_AI_Character_Toxic.BP_AI_Character_Toxic_C")
      (set `self.BehaviorTree` "/Game/Blueprints/AI/Behavior_Trees/AI_BT_Toxic.AI_BT_Toxic"))
    (:`NewEnumerator3`
      (set `self.AI_Class` "/Game/Blueprints/AI/AI_Characters/BP_AI_WhirlWind.BP_AI_WhirlWind_C")
      (set `self.BehaviorTree` "/Game/Blueprints/AI/Behavior_Trees/AI_BT_WhirlWind_Old.AI_BT_WhirlWind_Old")))
  (bind _returnvalue (`AIBlueprintHelperLibrary.SpawnAIFromClass` (`self.AI_Class`) (`self.BehaviorTree`) Location (struct) true))
  ;[1 1 1] Add altar reference to enemy
  (bind _asbase_enemy (cast `/Game/Blueprints/Combat_System/BaseEnemy` _returnvalue))
  (set `/Game/Blueprints/Combat_System/BaseEnemy.Altar_Ref` (`self.altar`) _asbase_enemy)
  (return _returnvalue))

(fn `SpawnWave`
  (params (waveNumber :type Integer))
  (locals (CurWave :type Integer) (enemiesList :type "Array of Pawn Object Reference"))
  (bind _output_get (set `local.CurWave` waveNumber))
  (bind (_value _returnvalue) (`BlueprintMapLibrary.Map_Find` (`self.wave`) _output_get))
  (if _returnvalue
    (for _array_element (`.Enemies_3_13C5F50D4D319F17D567209FAD5BFDB6` (break `/Game/Blueprints/Checkpoint_System/EnemiesArray` _value))
      (bind _returnvalue_2 (`self.SpawnOneEnemy` (`self.K2_GetActorLocation` (`|GetArrayItem` (`self.TargetPoints`) (`self.targetPointsIndex`))) _array_element))
      ;[1 1 1] Give enemy his wave number and add to enemies list
      (bind _asbase_enemy (cast `/Game/Blueprints/Combat_System/BaseEnemy` _returnvalue_2))
      (set `/Game/Blueprints/Combat_System/BaseEnemy.waveNumber` (`local.CurWave`) _asbase_enemy)
      (`KismetArrayLibrary.Array_Add` (`local.enemiesList`) _returnvalue_2)
      (`/Engine/EditorBlueprintResources/StandardMacros.IncrementInt` (`self.targetPointsIndex`)))
    ;[1 1 1] First wave
    (`/Game/Blueprints/Checkpoint_System/Altar.NewWave` (`self.altar`) (`local.CurWave`) (`local.enemiesList`))))

(fn `UserConstructionScript`)