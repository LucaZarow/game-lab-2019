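; Player pawn Blueprint handling axis movement, ranged orb fire, melee attacks and a damaging dash.
; Movement bindings include both world-axis and control-yaw-relative versions.
; BeginPlay attaches a weapon orb to a rotating spring arm, fired by shoot axes; attack and slash inputs spawn hitbox actors.
; Dash lerps the swept capsule forward on a timeline, damaging hit actors and briefly disabling their collision, with a delay-based cooldown.
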(event `InputAxis|MoveForward`
  (params (AxisValue :type "Float (single-precision)"))
  ;[1 1 1] Basic Player Movement
  (`|ExecutionSequence`
    (:`then_0`
      (`self.AddMovementInput` (1.0 0.0 0.0) AxisValue))
    (:`then_1`
      (bind _returnvalue (`KismetMathLibrary.MakeVector` AxisValue (stale `InputAxis|MoveRight` AxisValue)))
      (if (> (`KismetMathLibrary.VSize` _returnvalue) 0.0) :!label _label
        (`self.K2_SetActorRotation` (`KismetMathLibrary.Conv_VectorToRotator` _returnvalue))))))

(event `InputAxis|MoveRight`
  (params (AxisValue :type "Float (single-precision)"))
  ;[1 1 1] Basic Player Movement
  (`|ExecutionSequence`
    (:`then_0`
      (`self.AddMovementInput` (0.0 1.0 0.0) AxisValue))
    (:`then_1`
      (goto _label))))

(event `InputAxis|MoveForward` :!enabledstate Disabled
  (params (AxisValue :type "Float (single-precision)"))
  ;[1 1 1] Basic Player Movement
  (`self.AddMovementInput` (`KismetMathLibrary.GetForwardVector` (`KismetMathLibrary.MakeRotator` 0.0 0.0 (.yaw (`self.GetControlRotation`)))) AxisValue))

(event `self.ReceiveBeginPlay`
  (bind _orbtemp (`self.OrbTemp`))
  ;[1 1 1] Spawn Ranged Orb Object
  (`|ExecutionSequence`
    (:`then_0`
      (bind _returnvalue (`|SpawnActorFromClass` "/Game/Blueprints/RangedWeapon_Orb.RangedWeapon_Orb_C" (`SceneComponent.K2_GetComponentToWorld` _orbtemp) "Undefined" "OverrideRootScale" null null))
      (bind _output_get (set `self.Weapon_Orb` _returnvalue))
      (`self.K2_AttachToComponent` _output_get _orbtemp "None" "SnapToTarget" "SnapToTarget" "SnapToTarget" true))))

(event `self.ReceiveTick`
  (params (DeltaSeconds :type "Float (single-precision)"))
  ;[1 1 1] Rotatates Orb
  (`SceneComponent.K2_AddLocalRotation` (`self.SpringArm_Orb`) (`KismetMathLibrary.MakeRotator` 0.0 0.0 (* DeltaSeconds (`self.OrbRotationSpeed`))) false false))

(event `InputAxis|MoveRight` :!enabledstate Disabled
  (params (AxisValue :type "Float (single-precision)"))
  ;[1 1 1] Basic Player Movement
  (`self.AddMovementInput` (`KismetMathLibrary.GetRightVector` (`KismetMathLibrary.MakeRotator` 0.0 0.0 (.yaw (`self.GetControlRotation`)))) AxisValue))

(event `InputAxis|ShootUp`
  (params (AxisValue :type "Float (single-precision)"))
  (bind _weapon_orb (`self.Weapon_Orb`))
  ;[1 1 1] Ranged Attack 360 no scope
  (bind _returnvalue (`KismetMathLibrary.MakeVector` AxisValue (stale `InputAxis|ShootRight` AxisValue)))
  (if (> (`KismetMathLibrary.VSize` _returnvalue) 0.25) :!label _label_2
    (`/Game/Blueprints/RangedWeapon_Orb.PullTrigger` _weapon_orb (`KismetMathLibrary.Conv_VectorToRotator` _returnvalue))
    (else
      (`/Game/Blueprints/RangedWeapon_Orb.ReleaseTrigger` _weapon_orb))))

(event `InputAction|Attack`
  (params (Key :type "Key Structure"))
  ;[1 1 1] Attack
  (:`Pressed`
    (`|SpawnActorFromClass` "/Game/Blueprints/Melee/BP_Hitbox.BP_Hitbox_C" (`KismetMathLibrary.Conv_VectorToTransform` (`SceneComponent.K2_GetComponentLocation` (`self.Mesh`))) "Undefined" "OverrideRootScale" null null)))

(event `InputAxis|ShootRight`
  (params (AxisValue :type "Float (single-precision)"))
  ;[1 1 1] Ranged Attack 360 no scope
  (goto _label_2))

(event `InputAction|Slash`
  (params (Key :type "Key Structure"))
  ;[1 1 1] Slash
  (:`Pressed`
    (`|SpawnActorFromClass` "/Game/Blueprints/Melee/BP_SwordSlash.BP_SwordSlash_C" (`KismetMathLibrary.Conv_VectorToTransform` (`SceneComponent.K2_GetComponentLocation` (`self.Mesh`))) "Undefined" "OverrideRootScale" null null)))

(event `InputAction|Dash`
  (params (Key :type "Key Structure"))
  ;[1 1 1] Dash, Q key
  (:`Pressed`
    (if (`self.CanDash`)
      (`self.DashTrail`)
      (bind (_returnvalue _dashstartpos) (`self.CalcDashEndPos`))
      (`TimelineComponent.SetPlayRate` (`self.TimelineLerp`) (`self.DashSpeed`))
      (bind (_direction _newtrack_0) (`Timeline|TimelineLerp` :!via `PlayFromStart`)
        (:`Update`
          (bind _sweephitresult (`SceneComponent.K2_SetWorldLocation` (`self.CapsuleComponent`) (`KismetMathLibrary.VLerp` _dashstartpos _returnvalue _newtrack_0) true false))
          (bind (_output_get _hitactor) (`self.DashHitCalc` _sweephitresult))
          (if _output_get
            (`KismetSystemLibrary.Delay` 0.2)
            (`self.SetActorEnableCollision` _hitactor true))
          (set `self.CanDash` false)
          (`KismetSystemLibrary.Delay` 2.55)
          (set `self.CanDash` true))))))

(fn `CalcDashEndPos`
  (returns (ReturnValue :type "Vector Structure") (DashStartPos :type "Vector Structure"))
  (bind _dashstartpos (`self.DashStartPos`))
  ;[1 1 1] Dash, on release of Q key
  (set `self.DashStartPos` (`SceneComponent.K2_GetComponentLocation` (`self.CapsuleComponent`)))
  (return (+ _dashstartpos (* (`SceneComponent.GetForwardVector` (`self.CapsuleComponent`)) (`self.DashDistance`))) _dashstartpos))

(fn `DashHitCalc`
  (params (Hit :type "HitResult Structure (by ref)"))
  (returns (Output_Get :type Boolean) (HitActor :type "Actor Object Reference"))
  (locals (HitActorObj :type "Actor Object Reference"))
  (bind (_bblockinghit _binitialoverlap _time _distance _location _impactpoint _normal _impactnormal _physmat _hitactor) (`GameplayStatics.BreakHitResult` Hit))
  (if (`KismetSystemLibrary.IsValid` _hitactor)
    (bind _output_get (set `local.HitActorObj` _hitactor))
    (bind _returnvalue (`self.GetComponentByClass` _output_get "/Game/Blueprints/BaseActorBlueprint.BaseActorBlueprint_C"))
    (if (`KismetSystemLibrary.IsValid` _returnvalue)
      (`/Game/Blueprints/BaseActorBlueprint.Calculate Health` _returnvalue (* (`self.DashDamage`) -1))
      (`self.SetActorEnableCollision` (`local.HitActorObj`) false)
      (set `self.DashHitResult` true)
      (else
        (set `self.DashHitResult` false :!label _label)))
    (else
      (goto _label)))
  (return (`self.DashHitResult`) (`local.HitActorObj`)))

(fn `DashTrail`
  (`GameplayStatics.SpawnEmitterAttached` "/Game/Blueprints/DashTrail.DashTrail" (`self.Cylinder`)))

(fn `UserConstructionScript`)