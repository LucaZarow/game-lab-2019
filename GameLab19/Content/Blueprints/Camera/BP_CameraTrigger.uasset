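; Camera trigger actor that points the LookatCamera's look-ahead along the player's forward vector when BP_Player overlaps it.
; An AllowLookAhead gate closes after an overlap, and a three-second timer, restarted on every overlap, reopens it.
; Helper functions, not called here, exchange stored rotation and look-at option with the camera's current values.
; All camera access uses the first LookatCamera found in the level.
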(event `self.ReceiveActorBeginOverlap`
  (params (OtherActor :type "Actor Object Reference"))
  (if (`self.allowLookAhead`)
    (`self.SetCameraLookAhead` OtherActor)
    (set `self.allowLookAhead` false))
  (`KismetSystemLibrary.K2_SetTimer` null "ReAllowLookAhead" 3.0))

(fn `ReAllowLookAhead`
  (locals (value :type Integer))
  (set `self.allowLookAhead` true))

(fn `SetCameraLookAhead`
  (params (`Other Actor` :type "Actor Object Reference"))
  (bind _asbp_player (cast `/Game/Blueprints/BP_Player` `Other Actor`))
  (bind _outactors (`GameplayStatics.GetAllActorsOfClass` "/Game/Blueprints/Camera/LookatCamera.LookatCamera_C"))
  (set `/Game/Blueprints/Camera/LookatCamera.LookAheadVector` (`self.GetActorForwardVector` _asbp_player) (`|GetArrayItem` _outactors)))

(fn `SetCameraLookatOption`
  (bind _outactors (`GameplayStatics.GetAllActorsOfClass` "/Game/Blueprints/Camera/LookatCamera.LookatCamera_C"))
  (bind _output (`|GetArrayItem` _outactors))
  (set `self.TempLookatOption` (`/Game/Blueprints/Camera/LookatCamera.LookatOption` _output))
  (set `/Game/Blueprints/Camera/LookatCamera.LookatOption` (`self.CameraLookatOption`) _output)
  (set `self.CameraLookatOption` (`self.TempLookatOption`)))

(fn `SetCameraRotation`
  (bind _outactors (`GameplayStatics.GetAllActorsOfClass` "/Game/Blueprints/Camera/LookatCamera.LookatCamera_C"))
  (bind _output (`|GetArrayItem` _outactors))
  (set `self.TempRotation` (`SceneComponent.GetSocketRotation` (`CameraActor.CameraComponent` _output) "None"))
  (`self.K2_SetActorRotation` _output (`self.CameraRotation`) false)
  (set `self.CameraRotation` (`self.TempRotation`)))

(fn `UserConstructionScript`)