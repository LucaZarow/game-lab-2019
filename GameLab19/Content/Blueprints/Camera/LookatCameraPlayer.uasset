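; Camera actor that follows the player along a spline path, always looking at them and zooming by distance.
; BeginPlay caches the BP_Player pawn as the target after a brief delay.
; Each Tick eases the root toward the closest point to the player on CameraPath's spline, then snaps the camera's rotation onto the target.
; Target distance is normalized between near and far limits to drive a smoothly interpolated FOV.
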(event `self.ReceiveBeginPlay`
  (`KismetSystemLibrary.Delay` 0.01)
  (bind _asbp_player (cast `/Game/Blueprints/BP_Player` (`GameplayStatics.GetPlayerPawn` 0))
    (:`then`
      (set `self.TargetActor` _asbp_player))
    (:`CastFailed`
      (`KismetSystemLibrary.PrintString` "\"get player failed\""))))

(event `self.ReceiveTick`
  (params (DeltaSeconds :type "Float (single-precision)"))
  (`self.UpdateCameraPosition`)
  (`self.UpdateCameraLookat`)
  (`self.UpdateCameraDistance`)
  (`self.NormalizeDistance`)
  (`self.UpdateCameraFOV`))

(event `UpdateCameraLookat`
  (bind _targetactor (`self.TargetActor`))
  (bind _cameracomponent (`self.CameraComponent`))
  (`/Engine/EditorBlueprintResources/StandardMacros.IsValid` _targetactor
    (:`Is Valid`
      (`SceneComponent.K2_SetWorldRotation` _cameracomponent (`KismetMathLibrary.FindLookAtRotation` (`SceneComponent.K2_GetComponentLocation` _cameracomponent) (`self.K2_GetActorLocation` _targetactor)) false false))))

(fn `NormalizeDistance`
  (set `self.CurrentDistanceAlpha` (`KismetMathLibrary.FClamp` (`KismetMathLibrary.NormalizeToRange` (`self.Target Distance`) (`self.NearDist`) (`self.FarDist`)))))

(fn `UpdateCameraDistance`
  (set `self.Target Distance` (`self.GetDistanceTo` (`self.TargetActor`))))

(fn `UpdateCameraFOV`
  (bind _cameracomponent (`self.CameraComponent`))
  (`CameraComponent.SetFieldOfView` _cameracomponent (`KismetMathLibrary.FInterpTo` (`CameraComponent.FieldOfView` _cameracomponent) (`KismetMathLibrary.Lerp` (`self.NearFov`) (`self.FarFov`) (`self.CurrentDistanceAlpha`)) (`GameplayStatics.GetWorldDeltaSeconds`) (`self.FovSpeed`))))

(fn `UpdateCameraPosition`
  (`/Engine/EditorBlueprintResources/StandardMacros.IsValid` (`self.TargetActor`)
    (:`Is Valid`
      (`SceneComponent.K2_SetWorldLocation` (`self.RootComponent`) (`KismetMathLibrary.VInterpTo` (`SceneComponent.K2_GetComponentLocation` (`self.RootComponent`)) (`SplineComponent.FindLocationClosestToWorldLocation` (`self.GetComponentByClass` (`self.CameraPath`) "/Script/Engine.SplineComponent") (`self.K2_GetActorLocation` (`GameplayStatics.GetPlayerPawn` 0)) "World") (`GameplayStatics.GetWorldDeltaSeconds`) 4.0) true false))))

(fn `UserConstructionScript`)