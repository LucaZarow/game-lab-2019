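; LookatCamera is a rail camera that follows the player along a spline path.
; Each tick it eases toward the path point nearest the player, then aims by LookatOption at the nearest look-at spline point, the player, their midpoint, or a point actor.
; It also maps its distance to the player onto a near-to-far range to smoothly interpolate field of view.
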(event `self.ReceiveBeginPlay`
  ;[1 1 1] GetPlayer
  (`KismetSystemLibrary.Delay` 0.01)
  (bind _asbp_player (cast `/Game/Blueprints/BP_Player` (`GameplayStatics.GetPlayerPawn` 0))
    (:`then`
      (set `self.TargetActor` _asbp_player))
    (:`CastFailed`
      (`KismetSystemLibrary.PrintString` "\"get player failed\""))))

(event `self.ReceiveTick`
  (params (DeltaSeconds :type "Float (single-precision)"))
  ;[1 1 1] UpdateCameraParameters
  (`self.UpdateCameraPosition`)
  (`self.UpdateCameraLookat`)
  (`self.UpdateCameraDistance`)
  (`self.NormalizeDistance`)
  (`self.UpdateCameraFOV`))

(fn `NormalizeDistance`
  (set `self.CurrentDistanceAlpha` (`KismetMathLibrary.FClamp` (`KismetMathLibrary.NormalizeToRange` (`self.Target Distance`) (`self.NearDist`) (`self.FarDist`)))))

(fn `UpdateCameraDistance`
  (set `self.Target Distance` (`self.GetDistanceTo` (`self.TargetActor`))))

(fn `UpdateCameraFOV`
  (bind _cameracomponent (`self.CameraComponent`))
  (`CameraComponent.SetFieldOfView` _cameracomponent (`KismetMathLibrary.FInterpTo` (`CameraComponent.FieldOfView` _cameracomponent) (`KismetMathLibrary.Lerp` (`self.NearFov`) (`self.FarFov`) (`self.CurrentDistanceAlpha`)) (`GameplayStatics.GetWorldDeltaSeconds`) (`self.FovSpeed`))))

(fn `UpdateCameraLookat`
  (bind _cameracomponent (`self.CameraComponent`))
  (bind _cameracomponent_2 (`self.CameraComponent`))
  (bind _cameracomponent_3 (`self.CameraComponent`))
  (bind _lookatspline (`self.LookAtSpline`))
  (bind _targetactor (`self.TargetActor`))
  (bind _cameracomponent_4 (`self.CameraComponent`))
  (bind _lookatpoint (`self.LookAtPoint`))
  (bind _returnvalue (`self.K2_GetActorLocation` _targetactor))
  (bind _returnvalue_2 (`SceneComponent.K2_GetComponentLocation` _cameracomponent_2))
  (bind _returnvalue_3 (`SplineComponent.FindLocationClosestToWorldLocation` (`self.GetComponentByClass` _lookatspline "/Script/Engine.SplineComponent") _returnvalue_2 "World"))
  (switch `/Game/Blueprints/Camera/LookAtOption` (`self.LookatOption`)
    (:`NewEnumerator0`
      ;[1 1 1] Look at spline
      (`/Engine/EditorBlueprintResources/StandardMacros.IsValid` _lookatspline
        (:`Is Valid`
          (`SceneComponent.K2_SetWorldRotation` _cameracomponent_2 (`KismetMathLibrary.FindLookAtRotation` _returnvalue_2 _returnvalue_3) false false))
        (:`Is Not Valid`
          (`KismetSystemLibrary.PrintString` "PLEASE INPUT LOOK AT SPLINE"))))
    (:`NewEnumerator1`
      ;[1 1 1] Look at player
      (`/Engine/EditorBlueprintResources/StandardMacros.IsValid` _targetactor
        (:`Is Valid`
          (`SceneComponent.K2_SetWorldRotation` _cameracomponent_4 (`KismetMathLibrary.FindLookAtRotation` (`SceneComponent.K2_GetComponentLocation` _cameracomponent_4) _returnvalue) false false))))
    (:`NewEnumerator2`
      ;[1 1 1] Look at both
      (`/Engine/EditorBlueprintResources/StandardMacros.IsValid` _lookatspline
        (:`Is Valid`
          (`/Engine/EditorBlueprintResources/StandardMacros.IsValid` _targetactor
            (:`Is Valid`
              (`SceneComponent.K2_SetWorldRotation` _cameracomponent (`KismetMathLibrary.FindLookAtRotation` (`SceneComponent.K2_GetComponentLocation` _cameracomponent) (`KismetMathLibrary.GetVectorArrayAverage` (`|MakeArray` _returnvalue_3 _returnvalue))) false false))))))
    (:`NewEnumerator4`
      ;[1 1 1] LookAtPoint
      (`/Engine/EditorBlueprintResources/StandardMacros.IsValid` _lookatpoint
        (:`Is Valid`
          (`SceneComponent.K2_SetWorldRotation` _cameracomponent_3 (`KismetMathLibrary.FindLookAtRotation` (`SceneComponent.K2_GetComponentLocation` _cameracomponent_3) (`self.K2_GetActorLocation` _lookatpoint)) false false))))))

(fn `UpdateCameraPosition`
  (`/Engine/EditorBlueprintResources/StandardMacros.IsValid` (`self.TargetActor`)
    (:`Is Valid`
      (`SceneComponent.K2_SetWorldLocation` (`self.RootComponent`) (`KismetMathLibrary.VInterpTo` (`SceneComponent.K2_GetComponentLocation` (`self.RootComponent`)) (`SplineComponent.FindLocationClosestToWorldLocation` (`self.GetComponentByClass` (`self.CameraPath`) "/Script/Engine.SplineComponent") (`self.K2_GetActorLocation` (`GameplayStatics.GetPlayerPawn` 0)) "World") (`GameplayStatics.GetWorldDeltaSeconds`) 4.0) true false))))

(fn `UserConstructionScript`)