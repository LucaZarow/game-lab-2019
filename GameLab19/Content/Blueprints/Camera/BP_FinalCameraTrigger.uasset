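; BP_FinalCameraTrigger is a trigger actor that switches the camera to its final setup when the player enters it.
; On BP_Player overlap, it assigns the final camera path to the first LookatCamera found in the level and the final look-at spline to Point.
; It also enables collision on the final bounding box, which it disables at BeginPlay.
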(event `self.ReceiveBeginPlay`
  (bind _finalboundingbox (`self.FinalBoundingBox`))
  (`/Engine/EditorBlueprintResources/StandardMacros.IsValid` _finalboundingbox
    (:`Is Valid`
      (`self.SetActorEnableCollision` _finalboundingbox false))))

(event `self.ReceiveActorBeginOverlap`
  (params (OtherActor :type "Actor Object Reference"))
  (bind _finalboundingbox (`self.FinalBoundingBox`))
  (cast `/Game/Blueprints/BP_Player` OtherActor)
  (bind _outactors (`GameplayStatics.GetAllActorsOfClass` "/Game/Blueprints/Camera/LookatCamera.LookatCamera_C"))
  (set `/Game/Blueprints/Camera/LookatCamera.CameraPath` (`self.FinalCameraPath`) (`|GetArrayItem` _outactors))
  (set `/Game/Blueprints/Camera/CameraLookatPoint.Spline` (`self.FinalLookatSpline`) (`self.Point`))
  (`/Engine/EditorBlueprintResources/StandardMacros.IsValid` _finalboundingbox
    (:`Is Valid`
      (`self.SetActorEnableCollision` _finalboundingbox true))))

(fn `UserConstructionScript`)