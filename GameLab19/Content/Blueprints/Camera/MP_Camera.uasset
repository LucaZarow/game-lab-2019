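; Shared multiplayer camera that aims to frame up to four players, set as every player controller's view target shortly after BeginPlay.
; A fast looping timer sets spring arm length from the largest pairwise player distance, clamped and debug-printed.
; It also interpolates position toward the P1–P4 location sum divided by PlayersReference length.
; Invalid players count as zero, and the setup loop assigns None to P1–P4.
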(event `self.ReceiveBeginPlay`
  (`KismetSystemLibrary.Delay` 0.01)
  (`self.ClassSetup`)
  (`KismetSystemLibrary.K2_SetTimer` null "UpdateCamera" 0.001 true))

(event `UpdateCamera`
  (`self.SetArmLength`)
  (`self.SetCameraPos`))

(fn `CalculateDistance`
  (params (PlayerRef1 :type "Character Object Reference") (PlayerRef2 :type "Character Object Reference"))
  (returns (NewLocalVar_01 :type "Float (double-precision)"))
  (locals (Distance :type "Float (double-precision)" :default 0.0))
  (if (and (`KismetSystemLibrary.IsValid` PlayerRef1) (`KismetSystemLibrary.IsValid` PlayerRef2))
    (set `local.Distance` (`self.GetDistanceTo` PlayerRef1 PlayerRef2))
    (else
      (set `local.Distance` 0.0)))
  (return (`local.Distance`)))

(fn `ClassSetup`
  (bind _asmp_test_game_mode (cast `/Game/Blueprints/Camera/MP_Test_GameMode` (`GameplayStatics.GetGameMode`)))
  (set `self.GameMode` _asmp_test_game_mode)
  (bind _outactors (`GameplayStatics.GetAllActorsOfClass` "/Script/Engine.PlayerController"))
  (`PlayerController.SetViewTargetWithBlend` _outactors self 0.0 "VTBlend_Linear" 0.0 false)
  (for (_ _array_index) (`self.PlayersReference`)
    (switch `int` _array_index
      (:`0`
        (set `self.P1` null))
      (:`1`
        (set `self.P2` null))
      (:`2`
        (set `self.P3` null))
      (:`3`
        (set `self.P4` null)))))

(fn `GetLocation`
  (params (Player :type "Actor Object Reference"))
  (returns (PlayerLocation :type "Vector Structure"))
  (locals (Location :type "Vector Structure" :default (0.0 0.0 0.0)))
  (`/Engine/EditorBlueprintResources/StandardMacros.IsValid` Player
    (:`Is Valid`
      (set `local.Location` (`self.K2_GetActorLocation` Player)))
    (:`Is Not Valid`
      (set `local.Location` (0.0 0.0 0.0))))
  (return (`local.Location`)))

(fn `SetArmLength`
  (bind _p4 (`self.P4`))
  (bind _p1 (`self.P1`))
  (bind _p2 (`self.P2`))
  (bind _p3 (`self.P3`))
  (bind _output_get (set `SpringArmComponent.TargetArmLength` (`KismetMathLibrary.FClamp` (`.MaxValue` (`KismetMathLibrary.MaxOfFloatArray` (`|MakeArray` (`self.CalculateDistance` _p1 _p2) (`self.CalculateDistance` _p2 _p3) (`self.CalculateDistance` _p2 _p4) (`self.CalculateDistance` _p1 _p3) (`self.CalculateDistance` _p1 _p4) (`self.CalculateDistance` _p3 _p4)))) (`self.MinArmLength`) (`self.MaxArmLength`)) (`self.SpringArm`)))
  (`KismetSystemLibrary.PrintString` (`KismetStringLibrary.Conv_DoubleToString` _output_get)))

(fn `SetCameraPos`
  (set `self.TargetPos` (/ (+ (`self.GetLocation` (`self.P1`)) (`self.GetLocation` (`self.P2`)) (`self.GetLocation` (`self.P3`)) (`self.GetLocation` (`self.P4`))) (`KismetMathLibrary.Conv_IntToDouble` (`KismetArrayLibrary.Array_Length` (`self.PlayersReference`)))))
  (`self.K2_SetActorLocation` (`KismetMathLibrary.VInterpTo` (`self.PreviousPos`) (`self.TargetPos`) (`GameplayStatics.GetWorldDeltaSeconds`) (`self.InterpSpeed`)))
  (set `self.PreviousPos` (`self.K2_GetActorLocation`)))

(fn `UserConstructionScript`)