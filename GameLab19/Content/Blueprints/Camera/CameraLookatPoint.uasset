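; Camera look-at point actor that glides along a spline to follow a spot just ahead of the player pawn.
; Each tick it projects a point in front of the pawn's forward vector onto the closest location on the referenced Spline actor's SplineComponent.
; It then eases its root toward that location with VInterpTo and a swept move, smoothing the point's motion.
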(event `self.ReceiveTick`
  (params (DeltaSeconds :type "Float (single-precision)"))
  (bind _returnvalue (`GameplayStatics.GetPlayerPawn` 0))
  (`SceneComponent.K2_SetWorldLocation` (`self.RootComponent`) (`KismetMathLibrary.VInterpTo` (`SceneComponent.K2_GetComponentLocation` (`self.RootComponent`)) (`SplineComponent.FindLocationClosestToWorldLocation` (`self.GetComponentByClass` (`self.Spline`) "/Script/Engine.SplineComponent") (+ (`self.K2_GetActorLocation` _returnvalue) (* (`self.GetActorForwardVector` _returnvalue) 100.0)) "World") (`GameplayStatics.GetWorldDeltaSeconds`) 4.0) true false))

(fn `UserConstructionScript`)