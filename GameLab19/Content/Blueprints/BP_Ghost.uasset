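; BP_Ghost is a short-lived afterimage of the player, frozen in the pose held when it spawns.
; On BeginPlay it copies the player mesh's pose onto a PoseableMesh and gives each material slot a dynamic instance of GhostMaterial.
; OpacityTimeline then drives a scalar parameter on those instances, though its name is left as None, and destroys the actor when finished.
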(event `self.ReceiveBeginPlay`
  (bind _asbp_player (cast `/Game/Blueprints/BP_Player` (`GameplayStatics.GetPlayerPawn` 0)))
  (set `self.PlayerRef` _asbp_player)
  (`self.GhostTrail`))

(event `GhostTrail`
  (bind _poseablemesh (`self.PoseableMesh`))
  (for _ (`MeshComponent.GetMaterials` (`self.PoseableMesh`))
    (bind _returnvalue (`KismetMaterialLibrary.CreateDynamicMaterialInstance` "/Game/Blueprints/GhostMaterial.GhostMaterial"))
    (bind _returnvalue_2 (`KismetArrayLibrary.Array_Add` (`self.DynamicMats`) _returnvalue))
    (`PrimitiveComponent.SetMaterial` _poseablemesh _returnvalue_2 _returnvalue)
    (`PoseableMeshComponent.CopyPoseFromSkeletalComponent` _poseablemesh (`Character.Mesh` (`self.PlayerRef`))))
  (bind (_direction _newtrack_0) (`Timeline|OpacityTimeline` :!via `PlayFromStart`)
    (:`Update`
      (for _array_element (`self.DynamicMats`)
        (`MaterialInstanceDynamic.SetScalarParameterValue` _array_element "None" _newtrack_0)))
    (:`Finished`
      (`self.K2_DestroyActor`))))

(fn `UserConstructionScript`
  (`KismetArrayLibrary.Array_Clear` (`self.DynamicMats`)))