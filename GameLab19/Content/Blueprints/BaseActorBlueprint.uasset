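; Base actor Blueprint that gives an actor health, with damage, healing and a death check.
; The damage event truncates incoming damage to an integer for TakeDamage, which, like Heal, feeds a signed change into CalculateHealth.
; CalculateHealth clamps health between zero and MaxHealth and runs CheckDeath unless capped at the maximum.
; Death is only a placeholder debug print, and the ShowHealth health bar creation on BeginPlay is disabled.
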(event `self.ReceiveBeginPlay` :!enabledstate Disabled
  ;[1 1 1] Make Health Bar
  (if (`self.ShowHealth`)
    (bind _returnvalue (`|CreateWidget` "/Game/Blueprints/Melee/UI_HealthBar.UI_HealthBar_C" :!enabledstate Disabled))
    (`UserWidget.AddToViewport` _returnvalue 0 :!enabledstate Disabled)))

(event `TakeDamageEvent` :!enabledstate Disabled
  (params (Damage :type "Float (double-precision)") (DamageType :type "DamageType Object Reference") (InstigatedBy :type "Controller Object Reference") (DamageCauser :type "Actor Object Reference"))
  (`self.TakeDamage` (`KismetMathLibrary.FTrunc` Damage)))

(fn `Calculate Health`
  (params (Addition :type Integer))
  (bind _maxhealth (`self.MaxHealth`))
  (bind _output_get (set `self.CurrentHealth` (+ (`self.CurrentHealth`) Addition)))
  (if (< _output_get 0)
    (set `self.CurrentHealth` 0)
    (`self.Check Death` :!label _label)
    (elif (> _output_get _maxhealth)
      (set `self.CurrentHealth` _maxhealth)
      (else
        (goto _label)))))

(fn `Check Death`
  (if (<= (`self.CurrentHealth`) 0)
    (`KismetSystemLibrary.PrintString` "Pawn has died") ; This would call the death event
  ))

(fn `Heal`
  (params (Healling :type Integer))
  (`self.Calculate Health` Healling))

(fn `TakeDamage`
  (params (Damage :type Integer))
  (locals (NewLocalVar_0 :type String :default "Hello"))
  (`self.Calculate Health` (* Damage -1))
  (`KismetSystemLibrary.PrintString` (`KismetStringLibrary.Conv_IntToString` (`self.CurrentHealth`))))