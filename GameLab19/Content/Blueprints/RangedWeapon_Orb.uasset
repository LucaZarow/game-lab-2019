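; Orb ranged weapon that auto-fires Test_Projectile actors from its Sphere component while the trigger is held.
; PullTrigger stores the aim rotation, then fires immediately and starts a looping Fire timer at ProjPerSecond.
; A DoOnce ignores repeated pulls for firing until ReleaseTrigger clears the timer and resets it, though each pull still updates the rotation.
; Releasing and re-pulling fires immediately, with no cooldown check.
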(event `PullTrigger`
  (params (Rotation :type "Rotator Structure"))
  (set `self.ProjectileRotation` Rotation)
  (`/Engine/EditorBlueprintResources/StandardMacros.DoOnce` false :!label _label
    (:`Completed`
      (`self.Fire`)
      (`KismetSystemLibrary.K2_SetTimer` null "Fire" (/ 1.0 (`self.ProjPerSecond`)) true))))

(event `ReleaseTrigger`
  (`KismetSystemLibrary.K2_ClearTimer` null "Fire")
  (goto _label :!via `Reset`))

(event `Fire`
  (`|SpawnActorFromClass` "/Game/Blueprints/Attacking_Testing/Test_Projectile.Test_Projectile_C" (`KismetMathLibrary.MakeTransform` (`SceneComponent.K2_GetComponentLocation` (`self.Sphere`)) (`self.ProjectileRotation`)) "AlwaysSpawn" "OverrideRootScale" null 6 "NewEnumerator0" false null))

(fn `UserConstructionScript`)