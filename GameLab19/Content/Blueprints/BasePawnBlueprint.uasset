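; BasePawnBlueprint is a pawn Blueprint with basic health tracking and a placeholder death check.
; BeginPlay sets CurrentHealth to MaxHealth, and AnyDamage passes truncated damage to TakeDamage.
; TakeDamage sets CurrentHealth to damage minus current health, the reverse of the usual subtraction, then calls CheckDeath.
; CheckDeath only prints a death message, off screen, when health is strictly below zero.
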(event `self.ReceiveBeginPlay`
  (`|ExecutionSequence`
    (:`then_0`
      (set `self.CurrentHealth` (`self.MaxHealth`)))))

(event `self.ReceiveAnyDamage`
  (params (Damage :type "Float (single-precision)") (DamageType :type "DamageType Object Reference") (InstigatedBy :type "Controller Object Reference") (DamageCauser :type "Actor Object Reference"))
  (`self.TakeDamage` (`KismetMathLibrary.FTrunc` Damage)))

(fn `CheckDeath`
  (if (< (`self.CurrentHealth`) 0)
    (`KismetSystemLibrary.PrintString` "A pawn has died" false)))

(fn `TakeDamage`
  (params (addition :type Integer))
  (set `self.CurrentHealth` (- addition (`self.CurrentHealth`)))
  (`self.CheckDeath`))

(fn `UserConstructionScript`)