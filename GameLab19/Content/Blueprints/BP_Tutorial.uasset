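; Tutorial controller that scripts post-process tint, camera shake and demon spawns for the tutorial.
; BeginPlay sets the PPVolume's scene color tint alpha in code, as the editor doesn't expose it; DarkTint runs a timeline lerping it toward zero to darken the ending.
; SpawnFirstDemon spawns a BasicCreep at TargetPoint.
; CameraShakey plays a strong camera shake, calls CanPass on BoundingBox and spawns a creep at the same point.
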(event `self.ReceiveBeginPlay`
  ;[1 1 1] Set starting alpha of color tint in world (under misc color grading on post processing volume, but doesnt let you change alpha there)
  (bind _output_get (set `self.PPSettings` (`PostProcessVolume.Settings` (`self.PPVolume`))))
  (bind (_scenecolortint_r _scenecolortint_g _scenecolortint_b) (break `LinearColor` (break `PostProcessSettings` _output_get)))
  (bind _output_get_2 (set `self.PPSettings` (make `PostProcessSettings` :`SceneColorTint` (make `LinearColor` _scenecolortint_r _scenecolortint_g _scenecolortint_b 0.9))))
  (set `PostProcessVolume.Settings` _output_get_2 (`self.PPVolume`)))

(event `DarkTint`
  (bind (_scenecolortint_r _scenecolortint_g _scenecolortint_b _scenecolortint_a) (break `LinearColor` (break `PostProcessSettings` (`self.PPSettings`))))
  ;[1 1 1] Tinit color to dark to end tutorial
  (bind (_direction _newtrack_0) (`Timeline|Timeline_0` :!via `PlayFromStart`)
    (:`Update`
      (bind _output_get (set `self.PPSettings` (make `PostProcessSettings` :`SceneColorTint` (make `LinearColor` _scenecolortint_r _scenecolortint_g _scenecolortint_b (`KismetMathLibrary.Lerp` _scenecolortint_a 0.0 _newtrack_0)))))
      (set `PostProcessVolume.Settings` _output_get (`self.PPVolume`)))))

(event `SpawnFirstDemon`
  (`AIBlueprintHelperLibrary.SpawnAIFromClass` "/Game/Blueprints/AI/AI_Characters/BP_AI_BasicCreep.BP_AI_BasicCreep_C" "/Game/Blueprints/AI/Behavior_Trees/AI_BT_BasicCreep.AI_BT_BasicCreep" (`self.K2_GetActorLocation` (`self.TargetPoint`))))

(fn `CameraShakey`
  (`PlayerController.ClientStartCameraShake` :`self` (`GameplayStatics.GetPlayerController` 0) :`Shake` "/Game/Blueprints/CameraShakeTutorial.CameraShakeTutorial_C" :`Scale` 10.0)
  (`/Game/Blueprints/Checkpoint_System/BoundingBox.CanPass` (`self.BoundingBox`))
  (`AIBlueprintHelperLibrary.SpawnAIFromClass` "/Game/Blueprints/AI/AI_Characters/BP_AI_BasicCreep.BP_AI_BasicCreep_C" "/Game/Blueprints/AI/Behavior_Trees/AI_BT_BasicCreep.AI_BT_BasicCreep" (`self.K2_GetActorLocation` (`self.TargetPoint`))))

(fn `UserConstructionScript`)