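; Game mode that sets up a session on BeginPlay and handles pausing.
; It spawns and possesses a BP_Player for each player index at the PlayerStart tagged with that index, then triggers every BP_EnemySpawner.
; It adds the HUD and Twitch widgets, though a note marks the heart-bar switch as broken.
; Pausing shows a cached Pause_Menu with UI-only input, while unpausing removes all widgets and restores game input.
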(event `self.ReceiveBeginPlay`
  (`self.GetPlayerStartPoints`)
  (`self.SpawnPlayers`)
  (`self.SpawnEnemies`)
  (`self.SpawnUI` (`self.UsingHeartBar`)))

(fn `GetPlayerStartPoints`
  (bind _outactors (`GameplayStatics.GetAllActorsOfClass` "/Script/Engine.PlayerStart"))
  (set `self.PlayerStartArray` _outactors))

(fn `PauseGame`
  (bind _returnvalue (`GameplayStatics.GetPlayerController` 0))
  (`GameplayStatics.SetGamePaused` true)
  (`/Engine/EditorBlueprintResources/StandardMacros.IsValid` (`self.PauseMenu`)
    (:`Is Valid`
      _)
    (:`Is Not Valid`
      (bind _returnvalue_2 (`|CreateWidget` "/Game/Blueprints/UI/Pause_Menu.Pause_Menu_C" (`GameplayStatics.GetPlayerController` 0)))
      (bind _output_get (set `self.PauseMenu` _returnvalue_2))))
  (`UserWidget.AddToViewport` _output_get 0)
  (bind _resumebutton (`/Game/Blueprints/UI/Pause_Menu.ResumeButton` _output_get))
  (`WidgetBlueprintLibrary.SetInputMode_UIOnlyEx` (`GameplayStatics.GetPlayerController` 0) _resumebutton)
  (`Widget.SetUserFocus` _resumebutton _returnvalue)
  (set `PlayerController.bShowMouseCursor` true _returnvalue)
  (set `self.isPaused` true))

(fn `SetCurrentEnemy`
  (params (Enemy :type "Actor Object Reference"))
  (set `self.Current_Enemy` Enemy))

(fn `SpawnEnemies`
  (bind _outactors (`GameplayStatics.GetAllActorsOfClass` "/Game/Blueprints/AI/BP_EnemySpawner.BP_EnemySpawner_C"))
  (for _array_element _outactors
    (`/Game/Blueprints/AI/BP_EnemySpawner.SpawnEnemy` _array_element)))

(fn `SpawnPlayers`
  (for _index (range (`self.MaxPlayerCount`))
    (set `self.index` _index)
    (for _array_element (`self.PlayerStartArray`)
      (if (== (`PlayerStart.PlayerStartTag` _array_element) (`KismetStringLibrary.Conv_StringToName` (`KismetStringLibrary.Conv_IntToString` (`self.index`))))
        (bind _returnvalue (`|SpawnActorFromClass` "/Game/Blueprints/BP_Player.BP_Player_C" (`self.GetTransform` _array_element) "AlwaysSpawn" "OverrideRootScale" null null))
        (`KismetArrayLibrary.Array_AddUnique` (`self.Players`))
        (`Controller.Possess` (`GameplayStatics.GetPlayerController` (`self.index`)) _returnvalue)))))

(fn `SpawnUI`
  (params (UsingHeartBar :type Boolean))
  (bind _returnvalue (`|CreateWidget` "/Game/Blueprints/UI/UI_HeartBar.UI_HeartBar_C")) ; Change between UI_HealthBar and UI_HeartBar
  (bind _returnvalue_2 (`|CreateWidget` "/Game/Blueprints/UI/UI_Twitch.UI_Twitch_C"))
  (`UserWidget.AddToViewport` _returnvalue 0)
  (`UserWidget.AddToViewport` _returnvalue_2 0))

(fn `UnPauseGame`
  (bind _returnvalue (`GameplayStatics.GetPlayerController` 0))
  (`GameplayStatics.SetGamePaused` false)
  (`WidgetLayoutLibrary.RemoveAllWidgets`)
  (`WidgetBlueprintLibrary.SetInputMode_GameOnly` _returnvalue)
  (set `PlayerController.bShowMouseCursor` false _returnvalue)
  (set `self.isPaused` false))

(fn `UserConstructionScript`)