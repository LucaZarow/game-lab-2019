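; Player controller that turns input into camera-relative movement and combat actions for the controlled pawn.
; Movement follows the camera's flattened forward and right vectors, with facing derived from axis input offset by camera yaw.
; Melee, shoot, dash and jump call BP_Player; all but jump use flag-and-delay cooldowns, and attacks briefly lock movement with a timer.
; A testing button notifies and activates every AiManager's AIs.
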(event `InputAxis|MoveForward`
  (params (AxisValue :type "Float (single-precision)"))
  ;[1 1 1] Basic Player Movement
  (if (`self.CanMove`)
    (`|ExecutionSequence`
      (:`then_0`
        (`Pawn.AddMovementInput` (`self.K2_GetPawn`) (* (`KismetMathLibrary.Normal` (`KismetMathLibrary.MakeVector` (.x (`SceneComponent.GetForwardVector` (`PlayerCameraManager.TransformComponent` (`GameplayStatics.GetPlayerCameraManager` 0)))) (.y (`SceneComponent.GetForwardVector` (`PlayerCameraManager.TransformComponent` (`GameplayStatics.GetPlayerCameraManager` 0)))))) (`self.MovementSpeed`)) AxisValue false))
      (:`then_1`
        (bind _returnvalue (`KismetMathLibrary.MakeVector` AxisValue (stale `InputAxis|MoveRight` AxisValue)))
        (if (> (`KismetMathLibrary.VSize` _returnvalue) 0.0) :!label _label
          (`self.K2_SetActorRotation` (`KismetMathLibrary.Conv_VectorToRotator` _returnvalue) true)
          (`self.K2_AddActorWorldRotation` (`KismetMathLibrary.MakeRotator` 0.0 0.0 (.yaw (`SceneComponent.K2_GetComponentRotation` (`PlayerCameraManager.TransformComponent` (`GameplayStatics.GetPlayerCameraManager` 0))))))
          (`self.SetControlRotation` (`self.K2_GetActorRotation` (`self.K2_GetPawn`))))))))

(event `InputAxis|MoveRight`
  (params (AxisValue :type "Float (single-precision)"))
  ;[1 1 1] Basic Player Movement
  (if (`self.CanMove`)
    (`|ExecutionSequence`
      (:`then_0`
        (`Pawn.AddMovementInput` (`self.K2_GetPawn`) (* (`KismetMathLibrary.Normal` (`KismetMathLibrary.MakeVector` (.x (`SceneComponent.GetRightVector` (`PlayerCameraManager.TransformComponent` (`GameplayStatics.GetPlayerCameraManager` 0)))) (.y (`SceneComponent.GetRightVector` (`PlayerCameraManager.TransformComponent` (`GameplayStatics.GetPlayerCameraManager` 0)))))) (`self.MovementSpeed`)) AxisValue false))
      (:`then_1`
        (goto _label)))))

(event `InputAction|Attack`
  (params (Key :type "Key Structure"))
  (:`Pressed`
    (if (`self.CanMelee`)
      (bind _asbp_player (cast `/Game/Blueprints/BP_Player` (`self.K2_GetPawn`)))
      (set `self.CanMelee` false)
      (`/Game/Blueprints/BP_Player.AttackAction` _asbp_player)
      (`|ExecutionSequence`
        (:`then_0`
          (`KismetSystemLibrary.Delay` (`self.MeleeCooldown`))
          (set `self.CanMelee` true))
        (:`then_1`
          (set `self.CanMove` false)
          (`KismetSystemLibrary.K2_SetTimerDelegate` (delegate `EnanleMovement`) 0.4))))))

(event `InputAction|Shoot`
  (params (Key :type "Key Structure"))
  (:`Pressed`
    (if (`self.CanShoot`)
      (bind _asbp_player (cast `/Game/Blueprints/BP_Player` (`self.K2_GetPawn`)))
      (set `self.CanShoot` false)
      (`/Game/Blueprints/BP_Player.Fire V2` _asbp_player)
      (`|ExecutionSequence`
        (:`then_0`
          (`KismetSystemLibrary.Delay` (`self.RangeCooldown`))
          (set `self.CanShoot` true))
        (:`then_1`
          (set `self.CanMove` false)
          (`KismetSystemLibrary.K2_SetTimerDelegate` (delegate `EnanleMovement`) 0.3))))))

(event `EnanleMovement`
  (set `self.CanMove` true))

(event `InputAction|Dash`
  (params (Key :type "Key Structure"))
  (:`Pressed`
    (if (`self.CanDash`)
      (bind _asbp_player (cast `/Game/Blueprints/BP_Player` (`self.K2_GetPawn`)))
      (set `self.CanDash` false)
      (`/Game/Blueprints/BP_Player.DashAction` _asbp_player)
      (`KismetSystemLibrary.Delay` (`self.DashCooldown`))
      (set `self.CanDash` true))))

(event `InputAction|Jump`
  (params (Key :type "Key Structure"))
  (:`Pressed`
    (bind _asbp_player (cast `/Game/Blueprints/BP_Player` (`self.K2_GetPawn`)))
    (`/Game/Blueprints/BP_Player.Jump Action` _asbp_player)))

(event `InputAction|Testing Button`
  (params (Key :type "Key Structure"))
  (:`Pressed`
    (bind _outactors (`GameplayStatics.GetAllActorsOfClass` "/Game/Blueprints/AI/AiManager.AiManager_C"))
    (for _array_element _outactors
      (`/Game/Blueprints/AI/AiManager.Notify` _array_element)
      (`/Game/Blueprints/AI/AiManager.ActivateAIs` _array_element))))

(fn `UserConstructionScript`)