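; Test ranged player character with twin-stick style movement, shooting and dash.
; On BeginPlay it spawns a RangedWeapon_Orb and attaches it to the OrbTemp component.
; Move axes drive world-aligned movement and control rotation, while shoot axes pull or release the orb's trigger, both using a stick deadzone.
; Dash launches the character along camera forward rotated by control rotation when CanDash is true; its delayed stop is disabled.
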(event `self.ReceiveBeginPlay`
  (bind _orbtemp (`self.OrbTemp`))
  (`|ExecutionSequence`
    (:`then_0`
      (bind _returnvalue (`|SpawnActorFromClass` "/Game/Blueprints/RangedWeapon_Orb.RangedWeapon_Orb_C" (`SceneComponent.K2_GetComponentToWorld` _orbtemp) "Undefined" "OverrideRootScale" null null))
      (bind _output_get (set `self.Weapon_Orb` _returnvalue))
      (`self.K2_AttachToComponent` _output_get _orbtemp "None" "SnapToTarget" "SnapToTarget" "SnapToTarget" true))))

(event `InputAxis|MoveForward`
  (params (AxisValue :type "Float (single-precision)"))
  ;[1 1 1] Player Movement and rotation
  (`|ExecutionSequence`
    (:`then_0`
      (`self.AddMovementInput` (1.0 0.0 0.0) AxisValue))
    (:`then_1`
      (bind _returnvalue (`KismetMathLibrary.MakeVector` AxisValue (stale `InputAxis|MoveRight` AxisValue)))
      (if (> (`KismetMathLibrary.VSize` _returnvalue) 0.25) :!label _label
        (`Controller.SetControlRotation` (`self.GetController`) (`KismetMathLibrary.Conv_VectorToRotator` _returnvalue))))))

(event `InputAxis|ShootUp`
  (params (AxisValue :type "Float (single-precision)"))
  (bind _weapon_orb (`self.Weapon_Orb`))
  (bind _returnvalue (`KismetMathLibrary.MakeVector` AxisValue (stale `InputAxis|ShootRight` AxisValue)))
  (if (> (`KismetMathLibrary.VSize` _returnvalue) 0.25) :!label _label_2
    (`/Game/Blueprints/RangedWeapon_Orb.PullTrigger` _weapon_orb (`KismetMathLibrary.Conv_VectorToRotator` _returnvalue))
    (else
      (`/Game/Blueprints/RangedWeapon_Orb.ReleaseTrigger` _weapon_orb))))

(event `InputAxis|ShootRight`
  (params (AxisValue :type "Float (single-precision)"))
  (goto _label_2))

(event `InputAxis|MoveRight`
  (params (AxisValue :type "Float (single-precision)"))
  ;[1 1 1] Player Movement and rotation
  (`|ExecutionSequence`
    (:`then_0`
      (`self.AddMovementInput` (0.0 1.0 0.0) AxisValue))
    (:`then_1`
      (goto _label))))

(event `InputAction|Dash`
  (params (Key :type "Key Structure"))
  ;[1 1 1] Dash, on press of Q key
  (:`Pressed`
    (if (`self.CanDash`)
      (`self.LaunchCharacter` (* (`KismetMathLibrary.GreaterGreater_VectorRotator` (`SceneComponent.GetForwardVector` (`self.Camera`)) (`Controller.GetControlRotation` (`self.GetController`))) (`self.DashSpeed`)))
      (`KismetSystemLibrary.Delay` 0.05 :!enabledstate Disabled)
      (`MovementComponent.StopMovementImmediately` (`self.CharacterMovement`)))))

(fn `UserConstructionScript`)