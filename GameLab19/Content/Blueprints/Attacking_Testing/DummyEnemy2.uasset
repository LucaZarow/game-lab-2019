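; DummyEnemy2 is a test enemy character in the attack-testing folder that gets knocked back when another actor overlaps it.
; On overlap it prints a debug hit message, then launches itself horizontally away from the overlapping actor along the normalized, flattened direction between them.
; The launch overrides horizontal velocity and leaves vertical velocity intact.
; An AddMovementInput variant and an offset debug print remain unconnected.
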(event `self.ReceiveActorBeginOverlap` :!enabledstate Disabled
  (params (OtherActor :type "Actor Object Reference"))
  (`KismetSystemLibrary.PrintString` "Dummy 3 hit")
  (`self.LaunchCharacter` (* (`KismetMathLibrary.Normal` (`KismetMathLibrary.MakeVector` (.x (- (`self.K2_GetActorLocation`) (`self.K2_GetActorLocation` OtherActor))) (.y (- (`self.K2_GetActorLocation`) (`self.K2_GetActorLocation` OtherActor))))) 1000) true))

(fn `UserConstructionScript`)