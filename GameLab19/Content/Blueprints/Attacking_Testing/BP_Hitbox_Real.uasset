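; BP_Hitbox_Real is a short-lived hitbox actor, apparently for testing character attacks.
; On BeginPlay it casts its Spawner to BaseCharacter, snaps onto that character's mesh, then offsets mostly along local X and scales its root.
; It destroys itself after a brief delay, and the graph shown contains no overlap or damage logic.
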(event `self.ReceiveBeginPlay`
  ;[1 1 1] Create and scale hitbox
  (bind _asbase_character (cast `/Game/Blueprints/Attacking_Testing/BaseCharacter` (`self.Spawner`)))
  (`self.K2_AttachToComponent` (`Character.Mesh` _asbase_character) "None" "SnapToTarget" "KeepRelative" "KeepRelative")
  (`self.K2_AddActorLocalOffset` (80.0 0.0 10.0))
  (`SceneComponent.SetWorldScale3D` (`self.RootComponent`) (0.5 1.0 1.0))
  (`KismetSystemLibrary.Delay` 0.2)
  (`self.K2_DestroyActor`))

(fn `UserConstructionScript`)