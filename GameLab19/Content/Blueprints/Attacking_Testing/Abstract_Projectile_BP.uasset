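; Base projectile actor that damages characters of a different type than its attacker.
; On BeginPlay it waits out its Lifetime, then destroys itself.
; On overlap with a BaseCharacter whose type differs from AttackerType, it calls Damaged with HitBoxDamage and the attacker type, then destroys itself.
; Other overlaps are ignored, and the graphs contain no movement logic.
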(event `self.ReceiveBeginPlay`
  (`KismetSystemLibrary.Delay` (`self.Lifetime`))
  (`self.K2_DestroyActor`))

(event `self.ReceiveActorBeginOverlap`
  (params (OtherActor :type "Actor Object Reference"))
  (bind _attackertype (`self.AttackerType`))
  (bind _asbase_character (cast `/Game/Blueprints/Attacking_Testing/BaseCharacter` OtherActor))
  (if (`|EnumInequality` (`/Game/Blueprints/Attacking_Testing/BaseCharacter.CharcterType` _asbase_character) _attackertype)
    (`/Game/Blueprints/Attacking_Testing/BaseCharacter.Damaged` _asbase_character (`self.HitBoxDamage`) _attackertype)
    (`self.K2_DestroyActor`)))

(fn `UserConstructionScript`)