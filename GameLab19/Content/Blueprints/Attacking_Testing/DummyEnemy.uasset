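; DummyEnemy is a test enemy that reacts to contact with attack hitboxes.
; On BeginPlay it creates a UI_HealthBar widget and adds it to the viewport, without feeding it any values.
; Hit and overlap events share one path that prints debug text, checks for BP_Hitbox_Real and forces movement input along fixed world forward.
; The KnockBack event is empty, and the nodes for direction away from the attacker are unconnected.
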(event `self.ReceiveBeginPlay` :!enabledstate Disabled
  ;[1 1 1] Make Health Bar
  (bind _returnvalue (`|CreateWidget` "/Game/Blueprints/Melee/UI_HealthBar.UI_HealthBar_C"))
  (`UserWidget.AddToViewport` _returnvalue 0))

(event `KnockBack`
  (params (HitBox :type "Vector Structure")))

(event `self.ReceiveHit` :!enabledstate Disabled
  (params (MyComp :type "PrimitiveComponent Object Reference") (Other :type "Actor Object Reference") (OtherComp :type "PrimitiveComponent Object Reference") (bSelfMoved :type Boolean) (HitLocation :type "Vector Structure") (HitNormal :type "Vector Structure") (NormalImpulse :type "Vector Structure") (Hit :type "HitResult Structure (by ref)"))
  ;[1 1 1] Comment
  (`KismetSystemLibrary.PrintString` "Hit" :!label _label)
  (cast `/Game/Blueprints/Attacking_Testing/BP_Hitbox_Real` (stale `self.ReceiveActorBeginOverlap` OtherActor))
  (`KismetSystemLibrary.PrintString` "Hit by Hitbox")
  (`self.AddMovementInput` (`KismetMathLibrary.GetForwardVector` (struct)) 100.0 true))

(event `self.ReceiveActorBeginOverlap` :!enabledstate Disabled
  (params (OtherActor :type "Actor Object Reference"))
  (goto _label))

(fn `UserConstructionScript`)