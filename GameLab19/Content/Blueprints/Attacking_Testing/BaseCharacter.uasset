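; BaseCharacter is a base character Blueprint that provides health, typed damage, healing and knockback.
; Damaged ignores hits whose DamageType matches the character's own type; it and Heal both feed CalculateHealth, which clamps health and runs CheckDeath unless capped at maximum.
; Death only prints a message, and the health bar widget creation is disabled.
; GetLaunched pushes the character directly away from a launcher at a given force, overriding XY velocity.
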(event `CustomEvent`
  ;[1 1 1] Make Health Bar
  (if true
    (bind _returnvalue (`|CreateWidget` "/Game/Blueprints/Melee/UI_HealthBar.UI_HealthBar_C" :!enabledstate Disabled))
    (`UserWidget.AddToViewport` _returnvalue 0 :!enabledstate Disabled)))

(fn `Calculate Health`
  (params (addition :type Integer))
  (bind _maxhealth (`self.MaxHealth`))
  (bind _output_get (set `self.CurrentHealth` (+ (`self.CurrentHealth`) addition)))
  (if (< _output_get 0)
    (set `self.CurrentHealth` 0)
    (`self.Check Death` :!label _label)
    (elif (> _output_get _maxhealth)
      (set `self.CurrentHealth` _maxhealth)
      (else
        (goto _label)))))

(fn `Check Death`
  (if (<= (`self.CurrentHealth`) 0)
    (`KismetSystemLibrary.PrintString` "Pawn has died") ; This would call the death event
  ))

(fn `Damaged`
  (params (Damage :type Integer) (DamageType :type "/Game/Blueprints/Attacking_Testing/CharacterType Enum" :default "NewEnumerator0"))
  (if (`|EnumInequality` DamageType (`self.CharcterType`))
    (`self.Calculate Health` (* Damage -1))
    (`KismetSystemLibrary.PrintString` (`KismetStringLibrary.Conv_IntToString` (`self.CurrentHealth`)))))

(fn `GetLaunched`
  (params (Launcher :type "Actor Object Reference") (Launch_Force :type Integer :default 0))
  (`self.LaunchCharacter` (* (`KismetMathLibrary.Normal` (- (`self.K2_GetActorLocation`) (`self.K2_GetActorLocation` Launcher))) Launch_Force) true))

(fn `Heal`
  (params (Healing :type Integer))
  (`self.Calculate Health` Healing))

(fn `UserConstructionScript`)