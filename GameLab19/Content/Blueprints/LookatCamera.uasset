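; LookatCamera is a camera actor that keeps the player pawn in view by rotating toward it and zooming with distance.
; Each tick it snaps the camera component's rotation to the pawn, then normalises their distance into a clamped near-to-far alpha.
; That alpha blends between near and far FOV values, smoothed with FInterpTo.
; An offset-based position follow exists but is unconnected, so the actor never moves the camera.
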(event `self.ReceiveBeginPlay`
  (set `self.TargetActor` (`GameplayStatics.GetPlayerPawn` 0)))

(event `self.ReceiveTick`
  (params (DeltaSeconds :type "Float (single-precision)"))
  (`self.UpdateCameraLookat`)
  (`self.UpdateCameraDistance`)
  (`self.NormalizeDistance`)
  (`self.UpdateCameraFOV`))

(event `UpdateCameraLookat`
  (bind _cameracomponent (`self.CameraComponent`))
  (`SceneComponent.K2_SetWorldRotation` _cameracomponent (`KismetMathLibrary.FindLookAtRotation` (`SceneComponent.K2_GetComponentLocation` _cameracomponent) (`self.K2_GetActorLocation` (`self.TargetActor`))) false false))

(fn `NormalizeDistance`
  (set `self.CurrentDistanceAlpha` (`KismetMathLibrary.FClamp` (`KismetMathLibrary.NormalizeToRange` (`self.Target Distance`) (`self.NearDist`) (`self.FarDist`)))))

(fn `UpdateCameraDistance`
  (set `self.Target Distance` (`self.GetDistanceTo` (`self.TargetActor`))))

(fn `UpdateCameraFOV`
  (bind _cameracomponent (`self.CameraComponent`))
  (`CameraComponent.SetFieldOfView` _cameracomponent (`KismetMathLibrary.FInterpTo` (`CameraComponent.FieldOfView` _cameracomponent) (`KismetMathLibrary.Lerp` (`self.NearFov`) (`self.FarFov`) (`self.CurrentDistanceAlpha`)) (`GameplayStatics.GetWorldDeltaSeconds`) (`self.FovSpeed`))))

(fn `UpdateCameraPosition`)

(fn `UserConstructionScript`)