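; BP_Damaging is a melee hitbox actor that damages whatever it begins overlapping.
; On overlap it looks for a BaseActorBlueprint component on the other actor and, if found, calls Damaged with its stored damage and attacker type.
; SetStats sets both stored values.
; Older ApplyDamage and DummyEnemy knockback logic remains in the graph but is disconnected.
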(event `self.ReceiveActorBeginOverlap`
  (params (OtherActor :type "Actor Object Reference"))
  (bind _returnvalue (`self.GetComponentByClass` OtherActor "/Game/Blueprints/BaseActorBlueprint.BaseActorBlueprint_C"))
  ;[1 1 1] Apply damage to object
  (if true
    (`/Engine/EditorBlueprintResources/StandardMacros.IsValid` _returnvalue
      (:`Is Valid`
        (`/Game/Blueprints/BaseActorBlueprint.Damaged` _returnvalue (`self.HitBoxDamage`) (`self.AttackerType`))))))

(event `self.ReceiveActorEndOverlap`
  (params (OtherActor :type "Actor Object Reference"))
  ;[1 1 1] Apply damage to object
)

(fn `SetStats`
  (params (Damage :type Integer) (AttackType :type "/Game/Blueprints/Attacking_Testing/CharacterType Enum" :default "NewEnumerator0"))
  (set `self.HitBoxDamage` Damage)
  (set `self.AttackerType` AttackType))

(fn `UserConstructionScript`)